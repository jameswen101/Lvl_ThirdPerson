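; Train actor that moves its Body along the spline of a referenced Tracks actor, toggled between forward and reverse with the R key.
; A timeline's Alpha samples the spline transform by time to set world location and rotation.
; Each update sets play rate from TrainLapInSeconds and loops the timeline if the spline is closed.
; The construction script places the Body at StartPosition on the spline when Tracks is valid.
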(event `Key|R`
  (params (Key :type "Key Structure"))
  (:`Pressed`
    (`/Engine/EditorBlueprintResources/StandardMacros.FlipFlop`
      (:`A`
        (bind (_direction _alpha) (`Timeline|TrainMovementTimeline` :!label _label)
          (:`Update`
            (bind (_returnvalue_location _returnvalue_rotation) (`KismetMathLibrary.BreakTransform` (`SplineComponent.GetTransformAtTime` (`/Game/Blueprints/BP_TrainTracks.Spline` (`self.Tracks`)) _alpha "World" false false)))
            ;[1 1 1] Calculate Our Location on the Spline Based on % Alpha. Convet that to 3D Position and Rotation
            (`SceneComponent.K2_SetWorldLocationAndRotation` (`self.Body`) _returnvalue_location _returnvalue_rotation false false)
            ;[1 1 1] Set speed of the train by controlling timeline play rate (1/TrainLapInSeconds)
            (`TimelineComponent.SetPlayRate` (`self.TrainMovementTimeline`) (/ 1.0 (`KismetMathLibrary.FMax` (`self.TrainLapInSeconds`) 1e-05)))
            ;[1 1 1] Loop the timeline if the track loops
            (`TimelineComponent.SetLooping` (`self.TrainMovementTimeline`) (`SplineComponent.IsClosedLoop` (`/Game/Blueprints/BP_TrainTracks.Spline` (`self.Tracks`)))))))
      (:`B`
        (goto _label :!via `Reverse`)))))

(event `self.ReceiveTick`
  (params (DeltaSeconds :type "Float (single-precision)")))

(fn `UserConstructionScript`
  (bind _tracks (`self.Tracks`))
  (bind (_returnvalue_location _returnvalue_rotation) (`KismetMathLibrary.BreakTransform` (`SplineComponent.GetTransformAtTime` (`/Game/Blueprints/BP_TrainTracks.Spline` _tracks) (`self.StartPosition`) "World" false false)))
  ;[1 1 1] Make Sure It's Not Null
  (`/Engine/EditorBlueprintResources/StandardMacros.IsValid` _tracks
    (:`Is Valid`
      ;[1 1 1] Set The Train Starting Position Based on Our StartPosition Variable
      (`SceneComponent.K2_SetWorldLocationAndRotation` (`self.Body`) _returnvalue_location _returnvalue_rotation false false))))