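; BP_Food is a collectible food pickup that the Spark player character gathers for a puzzle.
; When BP_SparkCharacter_Player overlaps FoodCollider, it sets IsTouched and passes through a DoOnce so collection happens only once.
; It then hides itself rather than being destroyed and registers with the first BP_PuzzleController found in the level via AddFoodToArray.
; Debug prints report the pickup and the food's name.
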(event `self.FoodCollider.OnComponentBeginOverlap`
  (params (OverlappedComponent :type "PrimitiveComponent Object Reference") (OtherActor :type "Actor Object Reference") (OtherComp :type "PrimitiveComponent Object Reference") (OtherBodyIndex :type Integer) (bFromSweep :type Boolean) (SweepResult :type "HitResult Structure (by ref)"))
  ;[1 1 1] If Spark Touched the Food, Add It to the Array
  (cast `/Game/Gameplay/Characters/Player/BP_SparkCharacter_Player` OtherActor)
  (bind _output_get (set `self.IsTouched` true))
  (`KismetSystemLibrary.PrintString` "Food acquired")
  (if _output_get
    (`/Engine/EditorBlueprintResources/StandardMacros.DoOnce` false
      (:`Completed`
        (`self.SetActorHiddenInGame` true)
        (bind _outactors (`GameplayStatics.GetAllActorsOfClass` "/Game/Blueprints/BP_PuzzleController.BP_PuzzleController_C"))
        (bind _output_get_2 (set `self.PuzzleControllerRef` (`|GetArrayItem` _outactors)))
        (`/Game/Blueprints/BP_PuzzleController.AddFoodToArray` _output_get_2 self)
        (`KismetSystemLibrary.PrintString` (`KismetStringLibrary.Concat_StrStr` (`self.FoodName`) " added to array"))))))

(event `self.ReceiveActorBeginOverlap`
  (params (OtherActor :type "Actor Object Reference")))

(fn `UserConstructionScript`)