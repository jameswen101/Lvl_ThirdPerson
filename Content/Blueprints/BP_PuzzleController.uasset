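; BP_PuzzleController is the controller for a cooking puzzle, tracking the food and cooked pots Spark holds and revealing a key for completed orders.
; Events add items to food and pot arrays, setting possession flags, and a cleanup event removes those marked served.
; OrderArrived runs the order counters through a single loop, then unhides the key.
; L and M print held food and pot contents; PotTouched only casts.
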(event `AddPotToArray`
  (params (PotItem :type "/Game/Blueprints/BP_Pot Object Reference"))
  (bind _potarray (`self.PotArray`))
  ;[1 1 1] Add Pot Spark Finished Cooking with to Array, if !HasPot -> HasPot
  (`KismetArrayLibrary.Array_Add` _potarray PotItem)
  (if (> (`KismetArrayLibrary.Array_Length` _potarray) 0)
    (set `self.HasPot` true)))

(event `PotTouched`
  (params (PotTouched :type "/Game/Blueprints/BP_Pot Object Reference"))
  (cast `/Game/Blueprints/BP_Pot` PotTouched))

(event `AddFoodToArray`
  (params (FoodItem :type "/Game/Blueprints/BP_Food Object Reference"))
  (bind _foodarray (`self.FoodArray`))
  ;[1 1 1] Add Food Item Spark Touched to Array, if !HasFood -> HasFood
  (`KismetArrayLibrary.Array_Add` _foodarray FoodItem)
  (if (> (`KismetArrayLibrary.Array_Length` _foodarray) 0)
    (set `self.HasFood` true)))

(event `Key|L`
  (params (Key :type "Key Structure"))
  ;[1 1 1] Show Spark the Food He's Holding when L Pressed
  (:`Pressed`
    (for _array_element (`self.FoodArray`)
      (`KismetSystemLibrary.PrintString` (`/Game/Blueprints/BP_Food.FoodName` _array_element)))))

(event `OrderArrived`
  ;[1 1 1] Unlock Key after Spark Finishes All 4 Orders
  (while (and (> (`self.OrdersRemaining`) 0) (< (`self.OrdersServed`) 4))
    (`/Engine/EditorBlueprintResources/StandardMacros.DecrementInt` (`self.OrdersRemaining`)
      (:`  `
        (`/Engine/EditorBlueprintResources/StandardMacros.IncrementInt` (`self.OrdersServed`)))))
  (`self.SetActorHiddenInGame` (`self.Key`) false))

(event `CleanUpServedItems`
  ;[1 1 1] Remove Food from Array when Served
  (`|ExecutionSequence`
    (:`then_0`
      (for _array_element (`self.FoodArray`)
        (if (`/Game/Blueprints/BP_Food.IsServed` _array_element)
          (`KismetArrayLibrary.Array_RemoveItem` (`self.FoodArray`) _array_element))))
    (:`then_1`
      ;[1 1 1] Remove Pot from Array when Served
      (for _array_element_2 (`self.PotArray`)
        (if (`/Game/Blueprints/BP_Pot.IsServed` _array_element_2)
          (`KismetArrayLibrary.Array_RemoveItem` (`self.PotArray`)))))))

(event `Key|M`
  (params (Key :type "Key Structure"))
  ;[1 1 1] Show Spark What's in the Pots He's Holding when M Pressed
  (:`Pressed`
    (for _array_element (`self.PotArray`)
      (`KismetSystemLibrary.PrintString` (`/Game/Blueprints/BP_Food.FoodName` (`/Game/Blueprints/BP_Pot.FoodInPot` _array_element))))))

(fn `AddFoodToList`)

(fn `UserConstructionScript`)