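; BP_TrainTracks is an actor that builds train track along a spline.
; Its construction script adds a spline mesh component for each segment between neighbouring points, attaches it to the spline and matches the local locations and tangents.
; The event graph separately holds a debug test of a custom AND macro, which latches Q and Z presses and prints once after both have fired.
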(event `Key|Q`
  (params (Key :type "Key Structure"))
  (:`Pressed`
    (`self.My ANDMaco` :!label _label
      (:`A&B`
        (`KismetSystemLibrary.PrintString` "A AND B")))))

(event `Key|Z`
  (params (Key :type "Key Structure"))
  (:`Pressed`
    (goto _label :!via `B`)))

(fn `UserConstructionScript`
  (locals (LocalCurrentIndex :type Integer) (LocalSplineMesh :type "SplineMeshComponent Object Reference"))
  (bind _spline (`self.Spline`))
  (bind _localcurrentindex (`local.LocalCurrentIndex`))
  (bind (_location _tangent) (`SplineComponent.GetLocationAndTangentAtSplinePoint` _spline _localcurrentindex "Local"))
  (bind (_location_2 _tangent_2) (`SplineComponent.GetLocationAndTangentAtSplinePoint` _spline (+ _localcurrentindex 1) "Local"))
  ;[1 1 1] Loop through the spline points
  (for _index (range (+ (- (`SplineComponent.GetNumberOfSplinePoints` (`self.Spline`)) 2) 1))
    (set `local.LocalCurrentIndex` _index)
    ;[1 1 1] Create a spline mesh component and attach it to the spline
    (bind _returnvalue (`AddComponent|NODE_AddSplineMeshComponent-0` :`bManualAttachment` true))
    (bind _output_get (set `local.LocalSplineMesh` _returnvalue))
    (`SceneComponent.K2_AttachToComponent` _output_get (`self.Spline`) "None" "KeepRelative" "KeepRelative" "KeepRelative" true)
    ;[1 1 1] Set the Location and Tangents of the Spline Mesh
    (`SplineMeshComponent.SetStartAndEnd` (`local.LocalSplineMesh`) _location _tangent _location_2 _tangent_2 true)))