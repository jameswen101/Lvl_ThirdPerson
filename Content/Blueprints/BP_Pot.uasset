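; BP_Pot is a cooking pot in a food puzzle that accepts one food category.
; When the Spark player overlaps its sphere, an empty pot takes the first matching item from BP_PuzzleController's FoodArray.
; Pressing C starts a recursive one-second Delay countdown, after which the pot hides and adds itself to the controller.
; End-overlap handling is unfinished, and the respawn-after-serving logic is unconnected.
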(event `self.ReceiveBeginPlay`
  ;[1 1 1] Have the System Remember the Food Object's Original Position
  (set `self.OriginalPosition` (`self.K2_GetActorLocation`)))

(event `self.Sphere.OnComponentBeginOverlap`
  (params (OverlappedComponent :type "PrimitiveComponent Object Reference") (OtherActor :type "Actor Object Reference") (OtherComp :type "PrimitiveComponent Object Reference") (OtherBodyIndex :type Integer) (bFromSweep :type Boolean) (SweepResult :type "HitResult Structure (by ref)"))
  ;[1 1 1] Place the Correct Food Item in the Pot Once Spark Touches the Pot; Print Error if No Food of the Correct Type
  (cast `/Game/Gameplay/Characters/Player/BP_SparkCharacter_Player` OtherActor)
  (`KismetSystemLibrary.PrintString` "Pot touched")
  (if (not (`KismetSystemLibrary.IsValid` (`self.FoodInPot`)))
    (set `self.CanCook` true)
    (bind _outactors (`GameplayStatics.GetAllActorsOfClass` "/Game/Blueprints/BP_PuzzleController.BP_PuzzleController_C"))
    (`KismetSystemLibrary.PrintString` "Pot casting to puzzle controller success")
    (bind _foodarray (`/Game/Blueprints/BP_PuzzleController.FoodArray` (`|GetArrayItem` _outactors)))
    (for _array_element _foodarray
      (if (`|EnumEquality` (`/Game/Blueprints/BP_Food.Category` _array_element) (`self.AcceptedFoodType`))
        (set `self.FoundMatch` true)
        (set `self.FoodInPot` _array_element)
        (`KismetArrayLibrary.Array_RemoveItem` _foodarray _array_element)
        (`KismetSystemLibrary.PrintString` (`KismetStringLibrary.Concat_StrStr` (`/Game/Blueprints/BP_Food.FoodName` _array_element) " ready to cook. Press C to begin cooking"))
        (set `self.ReadyToCook` true)
        (set `self.CanReceiveInput` true)
        (break)))
    (else
      (`KismetSystemLibrary.PrintString` "There's already food in the pot!"))))

(event `self.Sphere.OnComponentEndOverlap`
  (params (OverlappedComponent :type "PrimitiveComponent Object Reference") (OtherActor :type "Actor Object Reference") (OtherComp :type "PrimitiveComponent Object Reference") (OtherBodyIndex :type Integer))
  ;[1 1 1] Place the Correct Food Item in the Pot Once Spark Touches the Pot; Print Error if No Food of the Correct Type
  ;;[1 1 1] Pending: Turn off Ability to Cook If Spark Leaves the Pot
  (cast `/Game/Gameplay/Characters/Player/BP_SparkCharacter_Player` OtherActor))

(event `Key|C`
  (params (Key :type "Key Structure"))
  ;[1 1 1] Cook the Food Item of the Correct Food Type
  (:`Pressed`
    (if (and (`self.ReadyToCook`) (`self.CanCook`) (`self.CanReceiveInput`))
      (`self.PotCountdown`))))

(event `PotCountdown`
  ;[1 1 1] Pot Countdown
  (`KismetSystemLibrary.PrintString` "Countdown activated successfully")
  (`KismetSystemLibrary.PrintString` (`KismetStringLibrary.Conv_IntToString` (`self.CookingCountdown`)) true true (struct :`G` 0.66 :`B` 1.0 :`A` 1.0) 1.5)
  (`KismetSystemLibrary.Delay` 1.0)
  (`/Engine/EditorBlueprintResources/StandardMacros.DecrementInt` (`self.CookingCountdown`)
    (:`  `
      (if (> (`self.CookingCountdown`) 0)
        (`self.PotCountdown`)
        (else
          (`KismetSystemLibrary.PrintString` "Cooking finished. Please bring it to the correct table.")
          (`self.SetActorHiddenInGame` true)
          (bind _outactors (`GameplayStatics.GetAllActorsOfClass` "/Game/Blueprints/BP_PuzzleController.BP_PuzzleController_C"))
          (`/Game/Blueprints/BP_PuzzleController.AddPotToArray` (`|GetArrayItem` _outactors) self)
          (set `self.ReadyToCook` false)
          (set `self.FoundMatch` false)
          (set `self.CanCook` false))))))

(fn `UserConstructionScript`)