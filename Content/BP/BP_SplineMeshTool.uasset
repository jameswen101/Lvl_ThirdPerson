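; BP_SplineMeshTool is a construction-script tool that populates a spline with copies of an input static mesh as spline mesh components.
; It divides the spline length by the mesh's bounding-box Z extent to set the segment count and spacing.
; Each segment takes local positions and tangents from the spline, though its start and end sample the same distance.
; The event graph holds only disabled placeholder events.
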(fn `UserConstructionScript`
  (bind _spline (`self.Spline`))
  (bind _spline_2 (`self.Spline`))
  (bind (_returnvalue_min _returnvalue_max) (break `Box` (`StaticMesh.GetBoundingBox` (`self.InputMesh`))))
  (set `self.MeshScale` (.z (- _returnvalue_max _returnvalue_min)))
  (for _index (range (+ (`KismetMathLibrary.FTrunc` (/ (`SplineComponent.GetSplineLength` (`self.Spline`)) (`self.MeshScale`))) 1))
    (bind _returnvalue (* _index (`self.MeshScale`)))
    (bind _returnvalue_2 (`SplineComponent.GetLocationAtDistanceAlongSpline` _spline _returnvalue "Local"))
    (bind _returnvalue_3 (`AddComponent|NODE_AddSplineMeshComponent-0` :`RelativeTransform` (`KismetMathLibrary.Conv_VectorToTransform` _returnvalue_2)))
    (bind _returnvalue_4 (`StaticMeshComponent.SetStaticMesh` _returnvalue_3 (`self.InputMesh`)))
    (bind _returnvalue_5 (* (`self.MeshScale`) _index))
    (`SplineMeshComponent.SetStartAndEnd` _returnvalue_3 _returnvalue_2 (`SplineComponent.GetTangentAtDistanceAlongSpline` _spline _returnvalue "Local") (`SplineComponent.GetLocationAtDistanceAlongSpline` _spline_2 _returnvalue_5 "Local") (`SplineComponent.GetTangentAtDistanceAlongSpline` _spline_2 _returnvalue_5 "Local") _returnvalue_4)))