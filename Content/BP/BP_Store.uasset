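; BP_Store is a configurable storefront actor that dresses itself as a trading post, bread shop, grocery or barber shop.
; Its construction script switches on StoreType, adding the matching sign mesh at SignPosition and child actors for the layout, stored in StoreLayout variables.
; Most types place one layout at LIPosition, while the barber shop places three at two table positions and an entrance.
; The event graph holds no active logic.
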(fn `UserConstructionScript`
  (bind _returnvalue (`SceneComponent.GetRelativeTransform` (`self.LIPosition`)))
  (bind _returnvalue_2 (`SceneComponent.GetRelativeTransform` (`self.SignPosition`)))
  (switch `/Game/BP/StoreType` (`self.StoreType`)
    (:`NewEnumerator0`
      (bind _returnvalue_3 (`AddComponent|NODE_AddStaticMeshComponent-1` :`RelativeTransform` _returnvalue_2))
      (`StaticMeshComponent.SetStaticMesh` _returnvalue_3 (`self.TradingPostSign`))
      (bind _returnvalue_4 (`AddComponent|NODE_AddChildActorComponent-3` :`RelativeTransform` (`SceneComponent.GetRelativeTransform` (`self.LIPosition`))))
      (set `self.StoreLayout1` _returnvalue_4))
    (:`NewEnumerator1`
      (bind _returnvalue_5 (`AddComponent|NODE_AddStaticMeshComponent-2` :`RelativeTransform` _returnvalue_2))
      (`StaticMeshComponent.SetStaticMesh` _returnvalue_5 (`self.BreadSign`))
      (bind _returnvalue_6 (`AddComponent|NODE_AddChildActorComponent-2` :`RelativeTransform` _returnvalue))
      (set `self.StoreLayout1` _returnvalue_6))
    (:`NewEnumerator2`
      (bind _returnvalue_7 (`AddComponent|NODE_AddStaticMeshComponent-3` :`RelativeTransform` _returnvalue_2))
      (`StaticMeshComponent.SetStaticMesh` _returnvalue_7 (`self.GrocerySign`))
      (bind _returnvalue_8 (`AddComponent|NODE_AddChildActorComponent-1` :`RelativeTransform` _returnvalue))
      (set `self.StoreLayout1` _returnvalue_8))
    (:`NewEnumerator3`
      (bind _returnvalue_9 (`AddComponent|NODE_AddStaticMeshComponent-4` :`RelativeTransform` _returnvalue_2))
      (`StaticMeshComponent.SetStaticMesh` _returnvalue_9 (`self.BarberSign`))
      (bind _returnvalue_10 (`AddComponent|NODE_AddChildActorComponent-4` :`RelativeTransform` (`SceneComponent.GetRelativeTransform` (`self.BarberTablePosition1`))))
      (set `self.StoreLayout1` _returnvalue_10)
      (bind _returnvalue_11 (`AddComponent|NODE_AddChildActorComponent-6` :`RelativeTransform` (`SceneComponent.GetRelativeTransform` (`self.BarberTablePosition2`))))
      (set `self.StoreLayout2` _returnvalue_11)
      (bind _returnvalue_12 (`AddComponent|NODE_AddChildActorComponent-7` :`RelativeTransform` (`SceneComponent.GetRelativeTransform` (`self.BarberEntrance`))))
      (set `self.StoreLayout3` _returnvalue_12))))