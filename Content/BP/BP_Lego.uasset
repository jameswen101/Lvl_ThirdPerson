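; BP_Lego is an unfinished procedural actor that, judging by its name, is meant to build a Lego-style brick from mesh components.
; The construction script loops over Rows and Columns, adding a static mesh at CubeLocation and storing its Z bounds extent in CylinderOffset.
; CubeLocation never changes in the live loop, so the meshes share one transform.
; The X-stepping logic is disconnected, CylinderOffset feeds nothing live, and the event graph is empty.
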(fn `UserConstructionScript`
  (locals (NewLocalVar :type "Float (double-precision)" :default 0.0))
  (for _ (range (`self.Rows`))
    (for _ (range (`self.Columns`))
      (bind _returnvalue (`AddComponent|NODE_AddStaticMeshComponent-0` :`RelativeTransform` (`self.CubeLocation`)))
      (bind _output_get (set `self.CylinderOffset` (.z (`.BoxExtent` (`KismetSystemLibrary.GetComponentBounds` _returnvalue))))))))