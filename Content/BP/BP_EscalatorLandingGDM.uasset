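; Generated dynamic mesh actor that builds a landing box with collision for a pair of escalators.
; On rebuild, it syncs Escalator2's mesh count and X position to Escalator1 when they differ, then places the box midway between them in Y, with offset and size variables.
; CallRebuild forces an immediate rebuild, then recreates a closed fence spline from the mesh's boundary-loop vertices.
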(event `self.OnRebuildGeneratedMesh`
  (params (TargetMesh :type "DynamicMesh Object Reference"))
  (bind _escalator1 (`self.Escalator1`))
  (bind _escalator2 (`self.Escalator2`))
  (bind _escalator2_2 (`self.Escalator2`))
  (bind (_returnvalue_x _returnvalue_y _returnvalue_z) (`KismetMathLibrary.BreakVector` (`self.K2_GetActorLocation` _escalator2)))
  (bind (_returnvalue_x_2 _returnvalue_y_2 _returnvalue_z_2) (`KismetMathLibrary.BreakVector` (`self.K2_GetActorLocation` _escalator1)))
  (bind _noofmeshes (`/Game/BP/BP_SplineToolEscalator.NoOfMeshes` _escalator1))
  (if (not (and (== _noofmeshes (`/Game/BP/BP_SplineToolEscalator.NoOfMeshes` _escalator2)) (== _returnvalue_x_2 _returnvalue_x)))
    (`self.K2_SetActorLocation` _escalator2_2 (`KismetMathLibrary.MakeVector` _returnvalue_x_2 _returnvalue_y _returnvalue_z) false false)
    (set `/Game/BP/BP_SplineToolEscalator.NoOfMeshes` _noofmeshes _escalator2_2))
  (`GeometryScriptLibrary_MeshPrimitiveFunctions.AppendBoxWithCollision` TargetMesh (struct) (`KismetMathLibrary.MakeTransform` (`KismetMathLibrary.MakeVector` (+ (`self.LandingForwardOffset`) _returnvalue_x_2) (/ (+ _returnvalue_y_2 _returnvalue_y) 2.0) (* (+ _returnvalue_z_2 50.0) 5.0))) (`self.LandingDepth`) (`self.LandingWidth`)))

(fn `CallRebuild`
  (`self.MarkForMeshRebuild` true)
  (`self.RebuildFenceSpline`))

(fn `RebuildFenceSpline`
  (bind _spline (`self.Spline`))
  (bind _returnvalue (`BaseDynamicMeshComponent.GetDynamicMesh` (`self.DynamicMeshComponent`)))
  (bind (_indexloops _pathloops) (`GeometryScriptLibrary_MeshSelectionQueryFunctions.GetMeshSelectionBoundaryLoops` _returnvalue))
  (`SplineComponent.ClearSplinePoints` _spline false)
  (for _array_element _pathloops
    (for _index (range (`GeometryScriptLibrary_PolyPathFunctions.GetPolyPathNumVertices` _array_element))
      (`SplineComponent.AddSplinePoint` _spline (`.ReturnValue` (`GeometryScriptLibrary_PolyPathFunctions.GetPolyPathVertex` _array_element _index)) "Local" false)))
  (`SplineComponent.SetClosedLoop` _spline true false)
  (`SplineComponent.UpdateSpline` _spline))

(fn `UserConstructionScript`)