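; Generated dynamic mesh actor that procedurally builds a fountain with Geometry Script whenever its mesh rebuilds.
; It stacks base, middle and top cylinders with a disc by advancing a Z transform, giving the disc a second material slot for lake water.
; It then spawns the NS_Fountain Niagara system at the raised transform and prints a total height.
; Disconnected box, noise, boolean and static-mesh baking nodes remain unused.
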(event `self.OnRebuildGeneratedMesh`
  (params (TargetMesh :type "DynamicMesh Object Reference"))
  (bind _fountaintransform (`self.FountainTransform`))
  (bind _baseheight (`self.BaseHeight`))
  (bind _bcylinderheight (`self.BCylinderHeight`))
  (bind _topcylinderheight (`self.TopCylinderHeight`))
  (bind _output_get (set `self.DynamicMesh` TargetMesh))
  (bind _returnvalue (`GeometryScriptLibrary_MeshPrimitiveFunctions.AppendCylinder` _output_get (struct) _fountaintransform (`self.BaseRadius`) _baseheight))
  (`GeometryScriptLibrary_MeshMaterialFunctions.SetMaterialIDForMeshSelection` _returnvalue)
  (bind _output_get_2 (set `self.FountainTransform` (`KismetMathLibrary.MakeTransform` (`KismetMathLibrary.MakeVector` 0.0 0.0 (+ (.z (.location _fountaintransform)) _baseheight)))))
  (bind _returnvalue_2 (`GeometryScriptLibrary_MeshPrimitiveFunctions.AppendCylinder` _returnvalue (struct) _output_get_2 (`self.BCylinderRadius`) _bcylinderheight))
  (`GeometryScriptLibrary_MeshMaterialFunctions.SetMaterialIDForMeshSelection` _returnvalue_2)
  (bind _output_get_3 (set `self.FountainTransform` (`KismetMathLibrary.MakeTransform` (`KismetMathLibrary.MakeVector` 0.0 0.0 (+ (.z (.location _output_get_2)) _bcylinderheight 20.0)))))
  (bind _returnvalue_3 (`GeometryScriptLibrary_MeshPrimitiveFunctions.AppendDisc` _returnvalue_2 (struct) _output_get_3 (`self.DiscRadius`)))
  (`GeometryScriptLibrary_MeshMaterialFunctions.SetMaterialIDForMeshSelection` _returnvalue_3 (struct) 1)
  (bind _returnvalue_4 (`GeometryScriptLibrary_MeshPrimitiveFunctions.AppendCylinder` _returnvalue_3 (struct) _output_get_3 (`self.TopCylinderRadius`) _topcylinderheight))
  (`GeometryScriptLibrary_MeshMaterialFunctions.SetMaterialIDForMeshSelection` _returnvalue_4)
  (bind _returnvalue_5 (+ (.z (.location _output_get_3)) _topcylinderheight))
  (bind _output_get_4 (set `self.FountainTransform` (`KismetMathLibrary.MakeTransform` (`KismetMathLibrary.MakeVector` 0.0 0.0 _returnvalue_5))))
  (bind _output_get_5 (set `self.TotalHeight` _returnvalue_5))
  (`KismetSystemLibrary.PrintString` (`KismetStringLibrary.Conv_DoubleToString` _output_get_5))
  (`NiagaraFunctionLibrary.SpawnSystemAttached` "/Game/Niagara/NS_Fountain.NS_Fountain" null "None" (.location _output_get_4) (struct) "KeepRelativeOffset")
  (`PrimitiveComponent.SetMaterial` (`self.DynamicMeshComponent`) 1 "/Game/Materials/M_Water_Lake.M_Water_Lake"))

(fn `BakeToStaticMesh`
  (params (TargetMesh :type "DynamicMesh Object Reference"))
  (for _index (range (+ (`self.Iterations`) 1))
    (`BaseDynamicMeshComponent.GetDynamicMesh` (`self.DynamicMeshComponent`))
    (set `self.RockSeed` _index)
    (bind _returnvalue (`BaseDynamicMeshComponent.GetDynamicMesh` (`self.DynamicMeshComponent`)))
    (`GeometryScriptLibrary_MeshMaterialFunctions.SetMaterialIDForMeshSelection` _returnvalue)))

(fn `UserConstructionScript`)