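; Generated dynamic mesh actor that procedurally builds a trophy from a box pedestal and a sphere.
; On rebuild it appends two boxes of different sizes, then copies the Perlin sphere static mesh and appends it at the sphere transform.
; Boolean, remesh and noise chains are disconnected leftovers.
; BakeToStaticMesh is an uncalled, partly wired rock-variant loop whose asset creation and random-color material steps never run.
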(event `self.OnRebuildGeneratedMesh`
  (params (TargetMesh :type "DynamicMesh Object Reference"))
  (bind _output_get (set `self.DynamicMesh` TargetMesh))
  (bind _returnvalue (`GeometryScriptLibrary_MeshPrimitiveFunctions.AppendBox` _output_get (struct) (`self.BoxTransform`) 62.5 62.5 25.0))
  (bind _returnvalue_2 (`GeometryScriptLibrary_MeshPrimitiveFunctions.AppendBox` _returnvalue (struct) (`self.BoxTransform`) 50.0 50.0))
  (bind _returnvalue_3 (`GeometryScriptLibrary_StaticMeshFunctions.CopyMeshFromStaticMeshV2` (`self.PerlinSphereMesh`))
    (:`Success`
      (bind _output_get_2 (set `self.To Dynamic Mesh` _returnvalue_3))
      (`GeometryScriptLibrary_MeshBasicEditFunctions.AppendMesh` _returnvalue_2 _output_get_2 (`self.SphereTransform`) false (struct :`CombineMode` "EnableAllMatching")))))

(fn `BakeToStaticMesh`
  (params (TargetMesh :type "DynamicMesh Object Reference"))
  (for _index (range (+ (`self.Iterations`) 1))
    (`BaseDynamicMeshComponent.GetDynamicMesh` (`self.DynamicMeshComponent`))
    (set `self.RockSeed` _index)
    (bind _returnvalue (`BaseDynamicMeshComponent.GetDynamicMesh` (`self.DynamicMeshComponent`)))
    (`GeometryScriptLibrary_MeshMaterialFunctions.SetMaterialIDForMeshSelection` _returnvalue)))

(fn `UserConstructionScript`)