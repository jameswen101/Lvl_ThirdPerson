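; Escalator builder tool that assembles steps and two handrails in the construction script; the event graph is empty.
; Spawns BP_EscalatorStepMoving child actors at intervals along the spline, adding spacing, rise and random offset/yaw.
; Two straight spline meshes span the first to last step positions, shifted to either side as handrails.
; EscalatorDirection is passed to each step and picks up or down materials for steps and handrails.
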(fn `UserConstructionScript`
  (bind _escalatordirection (`self.EscalatorDirection`))
  (bind _starttransform_location (`KismetMathLibrary.BreakTransform` (`self.StartTransform`)))
  (bind _endtransform_location (`KismetMathLibrary.BreakTransform` (`self.EndTransform`)))
  (bind _randomoffset (`self.RandomOffset`))
  (bind _returnvalue (- _endtransform_location _starttransform_location))
  ; Remove Old Escalator Meshes- Start from Scratch
  (`KismetArrayLibrary.Array_Clear` (`self.InputMesh`))
  (for _index (range (`self.NoOfMeshes`))
    (if (== _index 0)
      (bind _returnvalue_2 (`KismetMathLibrary.MakeTransform` (+ (.location (`SplineComponent.GetTransformAtDistanceAlongSpline` (`self.Spline`) (* _index (/ (`SplineComponent.GetSplineLength` (`self.Spline`)) (`self.NoOfMeshes`))) "Local" false)) (`KismetMathLibrary.MakeVector` (+ (* _index (`self.Spacing`)) (`KismetMathLibrary.RandomFloatInRange` _randomoffset (* _randomoffset -1.0))) 0.0 (* _index (`self.StepHeightOffset`)))) (`KismetMathLibrary.MakeRotator` 0.0 0.0 (`KismetMathLibrary.RandomFloatInRange` (`self.RandomJitter`)))))
      (set `self.StartTransform` _returnvalue_2))
    (if (== _index (- (`self.NoOfMeshes`) 1))
      (set `self.EndTransform` _returnvalue_2))
    ; Spawn Escalator Step
    (bind _returnvalue_3 (`AddComponent|NODE_AddChildActorComponent-0` :`RelativeTransform` _returnvalue_2))
    (`ChildActorComponent.SetChildActorClass` _returnvalue_3 "/Game/BP/BP_EscalatorStepMoving.BP_EscalatorStepMoving_C")
    (bind _asbp_escalator_step_moving (cast `/Game/BP/BP_EscalatorStepMoving` (`ChildActorComponent.ChildActor` _returnvalue_3))
      (:`then`
        (set `/Game/BP/BP_EscalatorStepMoving.EscalatorDirection` _escalatordirection _asbp_escalator_step_moving)
        (if (`|EnumEquality` _escalatordirection "NewEnumerator0")
          (bind _cube (`/Game/BP/BP_EscalatorStepMoving.Cube` _asbp_escalator_step_moving))
          (`PrimitiveComponent.CreateDynamicMaterialInstance` _cube 0 "/Game/BP/MI_EscalatorStepsUp.MI_EscalatorStepsUp" "None")
          (else
            (`PrimitiveComponent.CreateDynamicMaterialInstance` _cube 0 "/Game/BP/MI_EscalatorStepsDown.MI_EscalatorStepsDown" "None")))
        (`KismetArrayLibrary.Array_Add` (`self.InputMesh`) (`StaticMeshComponent.StaticMesh` _cube)))
      (:`CastFailed`
        (`KismetSystemLibrary.PrintString` "Cast failed"))))
  (`KismetSystemLibrary.PrintString` (`KismetStringLibrary.Conv_VectorToString` _returnvalue))
  (bind _output_get (set `self.Direction` (`KismetMathLibrary.Normal` _returnvalue)))
  (set `self.Distance` (`KismetMathLibrary.Vector_Distance` _starttransform_location _endtransform_location))
  (for _index_2 (range 2)
    (bind _returnvalue_4 (`AddComponent|NODE_AddSplineMeshComponent-2`))
    (`SplineMeshComponent.SetStartAndEnd` _returnvalue_4 _starttransform_location _output_get _endtransform_location _output_get true)
    (bind _output_get_2 (set `self.Rise` (.z (`.BoxExtent` (`self.GetActorBounds` false)))))
    (bind _output_get_3 (set `self.Angle` (`KismetMathLibrary.DegAtan` (/ _output_get_2 (`self.Distance`)))))
    (`SceneComponent.K2_SetRelativeRotation` _returnvalue_4 (`KismetMathLibrary.MakeRotator` 0.0) false false)
    (if (== _index_2 0)
      (bind _returnvalue_5 (`SceneComponent.K2_GetComponentLocation` _returnvalue_4))
      (`SceneComponent.K2_SetWorldLocation` _returnvalue_4 (+ _returnvalue_5 (`KismetMathLibrary.MakeVector` 0.0 (`self.HandrailOffset`))) false false)
      (set `self.RHandrailAngle` _output_get_3)
      (else
        (`SceneComponent.K2_SetWorldLocation` _returnvalue_4 (+ _returnvalue_5 (`KismetMathLibrary.MakeVector` 0.0 (* (`self.HandrailOffset`) -1.0))) false false)
        (set `self.LHandrailAngle` _output_get_3)
        (`SceneComponent.K2_SetRelativeRotation` _returnvalue_4 (`KismetMathLibrary.MakeRotator` 0.0) false false)))
    (if (`|EnumEquality` (`self.EscalatorDirection`) "NewEnumerator0")
      (`PrimitiveComponent.CreateDynamicMaterialInstance` _returnvalue_4 0 "/Game/BP/MI_EscalatorHandrailUp.MI_EscalatorHandrailUp" "None")
      (else
        (`PrimitiveComponent.CreateDynamicMaterialInstance` _returnvalue_4 0 "/Game/BP/MI_EscalatorHandrailDown.MI_EscalatorHandrailDown" "None")))))