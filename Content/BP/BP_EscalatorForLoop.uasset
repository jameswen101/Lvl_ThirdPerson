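; BP_EscalatorForLoop is an actor that generates escalator-style steps in its construction script, with an empty event graph.
; A loop over NumberOfSteps adds a static mesh component at StepSpawnLocation, seeded from the actor's world location but used as a relative transform.
; The SetStaticMesh call specifies no mesh.
; The node offsetting each step forward and up is disconnected, so all components share one transform.
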(fn `UserConstructionScript`
  (set `self.StepSpawnLocation` (`self.K2_GetActorLocation`))
  (for _ (range (`self.NumberOfSteps`))
    (bind _returnvalue (`AddComponent|NODE_AddStaticMeshComponent-0` :`RelativeTransform` (`KismetMathLibrary.Conv_VectorToTransform` (`self.StepSpawnLocation`))))
    (`StaticMeshComponent.SetStaticMesh` _returnvalue null)))