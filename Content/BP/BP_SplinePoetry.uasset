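; BP_SplinePoetry is a spline-driven actor that scatters randomly assembled text along a path, built in the construction script.
; It adds text render components at even distance intervals along the spline, with the count driven by NoOfMeshes.
; Each component's text appends random picks from the Value array.
; A random offset and yaw jitter transform is left unconnected, and the event graph is empty.
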(fn `UserConstructionScript`
  (bind _value (`self.Value`))
  (for _index (range (+ (`self.NoOfMeshes`) 1))
    (bind _returnvalue (`AddComponent|NODE_AddTextRenderComponent-0` :`RelativeTransform` (`KismetMathLibrary.MakeTransform` (.location (`SplineComponent.GetTransformAtDistanceAlongSpline` (`self.Spline`) (* _index (/ (`SplineComponent.GetSplineLength` (`self.Spline`)) (`self.NoOfMeshes`))) "Local" false)))))
    (`TextRenderComponent.K2_SetText` _returnvalue (`KismetTextLibrary.Conv_StringToText` (`KismetStringLibrary.Concat_StrStr` (`KismetTextLibrary.Conv_TextToString` (`KismetArrayLibrary.Array_Random` _value)) "" (`KismetTextLibrary.Conv_TextToString` (`KismetArrayLibrary.Array_Random` _value)) "" (`KismetTextLibrary.Conv_TextToString` (`KismetArrayLibrary.Array_Random` _value)))))))