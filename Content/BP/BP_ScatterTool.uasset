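; Scatter tool actor that spawns copies of a chosen static mesh at random spots when its construction script runs.
; It sizes its box from an editable extent, then loops over the mesh count, adding components at random local X/Y offsets with zero Z.
; Each iteration also line-traces vertically through random box points with debug drawing, but the hit is unused, so placement ignores both box and surface.
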(fn `UserConstructionScript`
  (bind _randomxoffset (`self.RandomXOffset`))
  (bind _randomyoffset (`self.RandomYOffset`))
  (bind _returnvalue (`KismetMathLibrary.RandomPointInBoundingBox` (`self.K2_GetActorLocation`) (`BoxComponent.GetUnscaledBoxExtent` (`self.Box`))))
  (`BoxComponent.SetBoxExtent` (`self.Box`) (`self.In Box Extent`) true)
  (for _ (range (+ (`self.NoOfMeshes`) 1))
    (`KismetSystemLibrary.LineTraceSingle` :`Start` (+ _returnvalue (0.0 0.0 500.0)) :`End` (- _returnvalue (0.0 0.0 500.0)) :`TraceChannel` "TraceTypeQuery1" :`DrawDebugType` "ForOneFrame")
    (bind _returnvalue_2 (`AddComponent|NODE_AddStaticMeshComponent-0` :`RelativeTransform` (`KismetMathLibrary.MakeTransform` (`KismetMathLibrary.MakeVector` (`KismetMathLibrary.RandomFloatInRange` _randomxoffset (* _randomxoffset -1.0)) (`KismetMathLibrary.RandomFloatInRange` _randomyoffset (* _randomyoffset -1.0))))))
    (`StaticMeshComponent.SetStaticMesh` _returnvalue_2 (`self.InputMesh`))))