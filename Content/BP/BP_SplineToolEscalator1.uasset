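; Spline-based escalator tool actor that spawns step mesh components along its spline at BeginPlay.
; The loop count comes from spline length over Spacing, while placement divides the length by NoOfMeshes, with random XY offset and yaw jitter.
; EscalatorDirection selects the up or down step material for each component.
; The construction script is empty, holding only disconnected copies of the spawn and material logic.
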(event `self.ReceiveBeginPlay`
  (bind _randomoffset (`self.RandomOffset`))
  (bind _returnvalue (* _randomoffset -1.0))
  (`KismetSystemLibrary.PrintString` "Escalator event graph running")
  (for _index (range (+ (`KismetMathLibrary.FTrunc` (/ (`SplineComponent.GetSplineLength` (`self.Spline`)) (`self.Spacing`))) 1))
    (bind _returnvalue_2 (`AddComponent|NODE_AddStaticMeshComponent-2` :`RelativeTransform` (`KismetMathLibrary.MakeTransform` (+ (.location (`SplineComponent.GetTransformAtDistanceAlongSpline` (`self.Spline`) (* _index (/ (`SplineComponent.GetSplineLength` (`self.Spline`)) (`self.NoOfMeshes`))) "Local" false)) (`KismetMathLibrary.MakeVector` (`KismetMathLibrary.RandomFloatInRange` _randomoffset _returnvalue) (`KismetMathLibrary.RandomFloatInRange` _randomoffset _returnvalue))) (`KismetMathLibrary.MakeRotator` 0.0 0.0 (`KismetMathLibrary.RandomFloatInRange` (`self.RandomJitter`))))))
    (if (`|EnumEquality` (`self.EscalatorDirection`) "NewEnumerator0")
      (`PrimitiveComponent.SetMaterial` _returnvalue_2 0 "/Game/BP/MI_EscalatorStepsUp.MI_EscalatorStepsUp")
      (else
        (`PrimitiveComponent.SetMaterial` _returnvalue_2 0 "/Game/BP/MI_EscalatorStepsDown.MI_EscalatorStepsDown")))
    (`StaticMeshComponent.SetStaticMesh` _returnvalue_2 (`StaticMeshComponent.StaticMesh` _returnvalue_2))))

(fn `UserConstructionScript`)