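; Spline scattering actor that places a set number of copies of an input actor at even intervals along its spline.
; The construction script picks the spawn mode from the input: static mesh actors become mesh components, while other actors with a mesh component become child actors of the same class.
; Each copy gets random XY offset and yaw jitter.
; Child actors containing a PCG component trigger its generation.
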(event EventBeginPlay)

(event Collision|EventActorBeginOverlap
  (params (OtherActor :type Actor%20Object%20Reference)))

(event EventTick
  (params (DeltaSeconds :type Float%20%28single-precision%29)))

(fn ConstructionScript
  (bind _inputactor (Variables|Default|GetInputActor))
  (bind _inputmesh (Variables|Default|GetInputMesh))
  (bind _randomoffset (Variables|Default|GetRandomOffset))
  (bind _randomjitter (Variables|Default|GetRandomJitter))
  (bind _returnvalue (* _randomoffset -1.0))
  ;[0.15 0.15 0.15 0.5] Assign Spawn Mode
  (Utilities|Array|Clear (Variables|Default|GetInputMesh))
  (bind _asstatic_mesh_actor (Utilities|Casting|CastToStaticMeshActor _inputactor)
    (:then
      (Variables|Default|SetSpawnMode "NewEnumerator0")
      (Utilities|Array|Add (Variables|Default|GetInputMesh) (Variables|/Script/Engine.StaticMeshComponent|GetStaticMesh (Variables|/Script/Engine.StaticMeshActor|GetStaticMeshComponent _asstatic_mesh_actor)))
      (for _index (range 0 (- (Variables|Default|GetNoOfMeshes) 1)) :!label _label
        (if (Utilities|Enum|Equal(Enum) (Variables|Default|GetSpawnMode) "NewEnumerator0")
          (bind _returnvalue_2 (AddComponent|AddStaticMeshComponent false (Math|Transform|MakeTransform (+ (.Location (Math|Transform|BreakTransform (Spline|GetTransformatDistanceAlongSpline (Variables|Default|GetSpline) (Math|Conversions|ToFloat(Integer) (* _index (/ (Spline|GetSplineLength (Variables|Default|GetSpline)) (Variables|Default|GetNoOfMeshes)))) "Local" false))) (Math|Vector|MakeVector (Math|Random|RandomFloatinRange _randomoffset _returnvalue) (Math|Random|RandomFloatinRange _randomoffset _returnvalue) 0.0)) (Math|Rotator|MakeRotator 0.0 0.0 (Math|Random|RandomFloatinRange _randomjitter (* _randomjitter -1.0))))))
          (Components|StaticMesh|SetStaticMesh _returnvalue_2 (Utilities|Array|Get(acopy) _inputmesh (Math|Random|RandomIntegerinRange 0 (- (Utilities|Array|Length _inputmesh) 1))))
          (else
            (bind _returnvalue_3 (AddComponent|AddChildActorComponent false (Math|Transform|MakeTransform (+ (.Location (Math|Transform|BreakTransform (Spline|GetTransformatDistanceAlongSpline (Variables|Default|GetSpline) (Math|Conversions|ToFloat(Integer) (* _index (/ (Spline|GetSplineLength (Variables|Default|GetSpline)) (Variables|Default|GetNoOfMeshes)))) "Local" false))) (Math|Vector|MakeVector (Math|Random|RandomFloatinRange _randomoffset _returnvalue) (Math|Random|RandomFloatinRange _randomoffset _returnvalue) 0.0)) (Math|Rotator|MakeRotator 0.0 0.0 (Math|Random|RandomFloatinRange _randomjitter (* _randomjitter -1.0))))))
            (ChildActorComponent|SetChildActorClass _returnvalue_3 (Variables|Default|GetSpawnActorClass))
            (if (Utilities|IsValid (Actor|GetComponentbyClass (Variables|/Script/Engine.ChildActorComponent|GetChildActor _returnvalue_3) "/Script/PCG.PCGComponent"))
              (Variables|Default|SetPCGClassName (Actor|GetComponentbyClass (Variables|/Script/Engine.ChildActorComponent|GetChildActor _returnvalue_3) "/Script/PCG.PCGComponent"))
              (PCG|Generate (Actor|GetComponentbyClass (Variables|/Script/Engine.ChildActorComponent|GetChildActor _returnvalue_3) "/Script/PCG.PCGComponent") true))))))
    (:CastFailed
      (if (Utilities|IsValid (Actor|GetComponentbyClass _inputactor "/Script/Engine.StaticMeshComponent"))
        (Variables|Default|SetSpawnMode "NewEnumerator1")
        (Variables|Default|SetSpawnActorClass (Utilities|GetClass _inputactor))
        (goto _label)))))