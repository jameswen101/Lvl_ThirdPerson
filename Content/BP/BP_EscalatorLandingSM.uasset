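; Escalator landing actor that places and scales a Cube platform between two referenced escalators.
; The construction script caches Escalator1's step count and end transform, clamps landing width and depth to minimums, then calls ResetLocation.
; ResetLocation copies Escalator1's step count to Escalator2 when count or X differs, centers the landing between their Y positions, and derives height from Escalator1's end transform.
; All logic runs at construction, with no active runtime events.
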(fn `ResetLocation`
  (bind _escalator1 (`self.Escalator1`))
  (bind _escalator2 (`self.Escalator2`))
  (bind (_returnvalue_x _returnvalue_y _returnvalue_z) (`KismetMathLibrary.BreakVector` (`self.K2_GetActorLocation` _escalator2)))
  (bind (_returnvalue_x_2 _returnvalue_y_2) (`KismetMathLibrary.BreakVector` (`self.K2_GetActorLocation` _escalator1)))
  (bind _noofmeshes (`/Game/BP/BP_SplineToolEscalator.NoOfMeshes` _escalator1))
  (bind _returnvalue (+ (`self.LandingForwardOffset`) _returnvalue_x_2))
  (bind _returnvalue_2 (/ (+ _returnvalue_y_2 _returnvalue_y) 2.0))
  (bind _returnvalue_3 (* (+ (.z (.location (`/Game/BP/BP_SplineToolEscalator.EndTransform` _escalator1))) (`self.ZMultiplier`)) 5.0))
  (if (not (and (== _noofmeshes (`/Game/BP/BP_SplineToolEscalator.NoOfMeshes` _escalator2)) (== _returnvalue_x_2 _returnvalue_x)))
    (`self.K2_SetActorLocation` (`KismetMathLibrary.MakeVector` _returnvalue_x_2 _returnvalue_y _returnvalue_z))
    (set `/Game/BP/BP_SplineToolEscalator.NoOfMeshes` _noofmeshes _escalator2))
  (`self.K2_SetActorLocation` (`KismetMathLibrary.MakeVector` _returnvalue _returnvalue_2 _returnvalue_3))
  (`SceneComponent.K2_SetWorldTransform` (`self.Cube`) (`KismetMathLibrary.MakeTransform` (`KismetMathLibrary.MakeVector` _returnvalue _returnvalue_2 _returnvalue_3) (struct) (`KismetMathLibrary.MakeVector` (`self.Landing Depth`) (`self.LandingWidth`) 1.0)) false false))

(fn `UserConstructionScript`
  (bind _minwidth (`self.MinWidth`))
  (bind _mindepth (`self.MinDepth`))
  (bind _escalator1 (`self.Escalator1`))
  (bind _escalator1_2 (`self.Escalator1`))
  (bind _noofmeshes (`/Game/BP/BP_SplineToolEscalator.NoOfMeshes` _escalator1_2))
  (bind _endtransform (`/Game/BP/BP_SplineToolEscalator.EndTransform` _escalator1_2))
  (set `self.E1NumOfSteps` (`/Game/BP/BP_SplineToolEscalator.NoOfMeshes` _escalator1))
  (set `self.E1EndTransform` (`/Game/BP/BP_SplineToolEscalator.EndTransform` _escalator1))
  (if (not (>= (`self.LandingWidth`) _minwidth))
    (set `self.LandingWidth` _minwidth))
  (if (not (>= (`self.Landing Depth`) _mindepth))
    (set `self.Landing Depth` _mindepth)
    (if (not (and (== _noofmeshes (`self.E1NumOfSteps`)) (== (`self.E1EndTransform`) _endtransform)))
      (set `self.E1NumOfSteps` _noofmeshes)
      (set `self.E1EndTransform` _endtransform)))
  (`self.ResetLocation`))