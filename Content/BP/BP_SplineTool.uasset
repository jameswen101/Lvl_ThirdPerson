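; Spline placement tool that scatters static meshes along a spline from its construction script.
; It spaces NoOfMeshes components evenly by spline length, each using a random mesh from the InputMesh array.
; Each gets a random X/Y offset and random yaw, ignoring spline rotation and scale.
; Randomness is unseeded, so the layout rerolls on every reconstruction; a Spacing-based count calculation is left unconnected.
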(fn `UserConstructionScript`
  (bind _inputmesh (`self.InputMesh`))
  (bind _randomoffset (`self.RandomOffset`))
  (bind _randomjitter (`self.RandomJitter`))
  (bind _returnvalue (* _randomoffset -1.0))
  (for _index (range (`self.NoOfMeshes`))
    (bind _returnvalue_2 (`AddComponent|NODE_AddStaticMeshComponent-0` :`RelativeTransform` (`KismetMathLibrary.MakeTransform` (+ (.location (`SplineComponent.GetTransformAtDistanceAlongSpline` (`self.Spline`) (* _index (/ (`SplineComponent.GetSplineLength` (`self.Spline`)) (`self.NoOfMeshes`))) "Local" false)) (`KismetMathLibrary.MakeVector` (`KismetMathLibrary.RandomFloatInRange` _randomoffset _returnvalue) (`KismetMathLibrary.RandomFloatInRange` _randomoffset _returnvalue))) (`KismetMathLibrary.MakeRotator` 0.0 0.0 (`KismetMathLibrary.RandomFloatInRange` _randomjitter (* _randomjitter -1.0))))))
    (`StaticMeshComponent.SetStaticMesh` _returnvalue_2 (`|GetArrayItem` _inputmesh (`KismetMathLibrary.RandomIntegerInRange` 0 (- (`KismetArrayLibrary.Array_Length` _inputmesh) 1))))))