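; Geometry Script generated mesh actor that builds a fence piece procedurally and can bake it to static mesh assets.
; On rebuild it randomly bumps the stored radius, appends three cylinders with different transforms, displaces them by a noise texture, then solidifies the result.
; BakeToStaticMesh loops over the Meshes count, saving the current dynamic mesh as indexed assets without rebuilding between saves.
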(event EventBeginPlay)

(event Collision|EventActorBeginOverlap
  (params (OtherActor :type Actor%20Object%20Reference)))

(event EventTick
  (params (DeltaSeconds :type Float%20%28single-precision%29)))

(event Events|EventOnRebuildGeneratedMesh
  (params (TargetMesh :type Dynamic%20Mesh%20Object%20Reference))
  (bind _output_get (Variables|Default|SetRadius (Math|Random|RandomFloatinRange (Variables|Default|GetRadius) (+ (Variables|Default|GetRadius) 5.0))))
  (bind _returnvalue (GeometryScript|Primitives|AppendCylinder :TargetMesh TargetMesh :Radius _output_get :Height (Variables|Default|GetHeight) :RadialSteps (Variables|Default|GetRadialSteps) :HeightSteps (Variables|Default|GetSegments)))
  (bind _returnvalue_2 (GeometryScript|Primitives|AppendCylinder :TargetMesh _returnvalue :Transform (Math|Transform|MakeTransform (Math|Vector|MakeVector 0.0 0.0 (+ (Variables|Default|GetOffset) (Variables|Default|GetRadius))) (Math|Rotator|MakeRotator 0.0 9e+01 0.0) "1.000000,1.000000,1.000000") :Radius (Variables|Default|GetRadius) :Height (Variables|Default|GetHeight) :RadialSteps (Variables|Default|GetRadialSteps) :HeightSteps (Variables|Default|GetSegments)))
  (bind _returnvalue_3 (GeometryScript|Primitives|AppendCylinder :TargetMesh _returnvalue_2 :Transform (Math|Transform|MakeTransform (Math|Vector|MakeVector 0.0 0.0 (* (Variables|Default|GetHeight) 0.5)) "90.000000,0.000000,0.000000" "1.000000,1.000000,1.000000") :Radius (Variables|Default|GetRadius) :Height (Variables|Default|GetHeight) :RadialSteps (Variables|Default|GetRadialSteps) :HeightSteps (Variables|Default|GetSegments)))
  (bind _returnvalue_4 (Class|GeometryScriptLibraryMeshDeformFunctions|ApplyDisplacefromTextureMap :TargetMesh _returnvalue_3 :Texture (Variables|Default|GetNoiseTexture) :Options (Utilities|Struct|MakeGeometryScriptDisplaceFromTextureOptions (Variables|Default|GetNoiseMagnitude) (Variables|Default|GetNoiseScale) "(X=0.000000,Y=0.000000)" 0.5 0 "FullMeshSelection")))
  (Class|GeometryScriptLibraryMeshVoxelFunctions|ApplyMeshSolidify _returnvalue_4))

(fn ConstructionScript)

(fn BaketoStaticMesh
  (for _index (range 0 (Variables|Default|GetMeshes))
    (bind _returnvalue (DynamicMeshComponent|GetDynamicMesh (Variables|DynamicMeshActor|GetDynamicMeshComponent)))
    (GeometryScript|AssetManagement|CreateNewStaticMeshAssetfromMesh _returnvalue (Utilities|String|Append "/Game/PCG/Class08/Fence" "SM_Fence" (Utilities|String|ToString(Integer) _index)) (Utilities|Struct|MakeGeometryScriptCreateNewStaticMeshAssetOptions false false false "(bEnabled=False,bExplicitTangents=False,bLerpUVs=True,bSeparable=False,bVoxelNDF=True,bVoxelOpacity=False,ShapePreservation=None,PositionPrecision=-2147483648,NormalPrecision=-1,TangentPrecision=-1,BoneWeightPrecision=-1,TargetMinimumResidencyInKB=0,KeepPercentTriangles=1.000000,TrimRelativeError=0.000000,GenerateFallback=PlatformDefault,FallbackTarget=Auto,FallbackPercentTriangles=1.000000,FallbackRelativeError=1.000000,MaxEdgeLengthFactor=0.000000,NumRays=64,VoxelLevel=0,RayBackUp=0.000000,DisplacementUVChannel=0,DisplacementMaps=,NaniteAssemblyData=(Parts=,Nodes=))" 0.0 true "CTF_UseDefault" false))))