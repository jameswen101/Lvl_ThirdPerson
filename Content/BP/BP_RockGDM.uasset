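; BP_RockGDM is a generated dynamic mesh actor that procedurally builds a rock with Geometry Script.
; On rebuild it appends sphere-boxes and a box, then applies a boolean union, plane cut, uniform remesh, texture displacement and Perlin noise.
; BakeToStaticMesh then loops over Iterations, setting RockSeed and material IDs.
; Its static mesh asset creation and random-color material nodes are disconnected, so no assets are saved.
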(event `self.OnRebuildGeneratedMesh`
  (params (TargetMesh :type "DynamicMesh Object Reference"))
  (bind _output_get (set `self.DynamicMesh` TargetMesh))
  (bind _returnvalue (`GeometryScriptLibrary_MeshPrimitiveFunctions.AppendSphereBox` _output_get (struct) (`self.SphereTransform`)))
  (bind _returnvalue_2 (`GeometryScriptLibrary_MeshPrimitiveFunctions.AppendSphereBox` _returnvalue (struct) (`self.SphereTransform`)))
  (bind _returnvalue_3 (`GeometryScriptLibrary_MeshPrimitiveFunctions.AppendBox` _returnvalue_2 (struct) (`self.BoxTransform`)))
  (bind _returnvalue_4 (`GeometryScriptLibrary_MeshBooleanFunctions.ApplyMeshBoolean` _returnvalue_3 (struct) null (struct) "Union"))
  (bind _returnvalue_5 (`GeometryScriptLibrary_MeshBooleanFunctions.ApplyMeshPlaneCut` _returnvalue_4))
  (bind _returnvalue_6 (`GeometryScriptLibrary_RemeshingFunctions.ApplyUniformRemesh` _returnvalue_5))
  (bind _returnvalue_7 (`GeometryScriptLibrary_MeshDeformFunctions.ApplyDisplaceFromTextureMap` _returnvalue_6))
  (bind _returnvalue_8 (`GeometryScriptLibrary_MeshDeformFunctions.ApplyPerlinNoiseToMesh2` _returnvalue_7 (struct) (make `GeometryScriptPerlinNoiseOptions` (make `GeometryScriptPerlinNoiseLayerOptions` 5.0))))
  (`self.BakeToStaticMesh` _returnvalue_8))

(fn `BakeToStaticMesh`
  (params (TargetMesh :type "DynamicMesh Object Reference"))
  (for _index (range (+ (`self.Iterations`) 1))
    (`BaseDynamicMeshComponent.GetDynamicMesh` (`self.DynamicMeshComponent`))
    (set `self.RockSeed` _index)
    (bind _returnvalue (`BaseDynamicMeshComponent.GetDynamicMesh` (`self.DynamicMeshComponent`)))
    (`GeometryScriptLibrary_MeshMaterialFunctions.SetMaterialIDForMeshSelection` _returnvalue)))

(fn `UserConstructionScript`)