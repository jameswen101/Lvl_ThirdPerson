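; BP_SpacingSplineSpawner is a construction-time tool that places copies of a chosen mesh at regular intervals along a spline.
; The construction script divides the spline length by Spacing to set the copy count, then adds a static mesh component at each distance step.
; Each component follows the spline's local position and rotation, ignores spline scale, and displays InputMesh.
; The event graph holds no runtime logic.
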(fn `UserConstructionScript`
  (for _index (range (+ (`KismetMathLibrary.FTrunc` (/ (`SplineComponent.GetSplineLength` (`self.Spline`)) (`self.Spacing`))) 1))
    (bind _returnvalue (`AddComponent|NODE_AddStaticMeshComponent-0` :`RelativeTransform` (`SplineComponent.GetTransformAtDistanceAlongSpline` (`self.Spline`) (* _index (`self.Spacing`)) "Local" false)))
    (`StaticMeshComponent.SetStaticMesh` _returnvalue (`self.InputMesh`))))