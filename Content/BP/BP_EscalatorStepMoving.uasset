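; BP_EscalatorStepMoving is an escalator step actor that picks its Cube material to match the escalator's direction.
; The construction script checks EscalatorDirection and creates a dynamic material instance from the Up or Down steps material.
; A SetMaterial function makes the same choice but assigns the material directly.
; The event graph holds no active logic, so the Blueprint itself moves nothing at runtime.
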(fn `SetMaterial`
  (if (`|EnumEquality` (`self.EscalatorDirection`) "NewEnumerator0")
    (`PrimitiveComponent.SetMaterial` (`self.Cube`) 0 "/Game/BP/MI_EscalatorStepsUp.MI_EscalatorStepsUp")
    (else
      (`PrimitiveComponent.SetMaterial` (`self.Cube`) 0 "/Game/BP/MI_EscalatorStepsDown.MI_EscalatorStepsDown"))))

(fn `UserConstructionScript`
  (if (`|EnumEquality` (`self.EscalatorDirection`) "NewEnumerator0")
    (`PrimitiveComponent.CreateDynamicMaterialInstance` (`self.Cube`) 0 "/Game/BP/MI_EscalatorStepsUp.MI_EscalatorStepsUp" "None")
    (else
      (`PrimitiveComponent.CreateDynamicMaterialInstance` (`self.Cube`) 0 "/Game/BP/MI_EscalatorStepsDown.MI_EscalatorStepsDown" "None"))))