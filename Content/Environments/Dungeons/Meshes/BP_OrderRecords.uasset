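; BP_OrderRecords is an order record actor that prints the food orders of every table to screen when any actor begins overlapping it.
; It gathers all SM_Prop_Table_4_Blueprint actors and prints each table number, followed by its order requirements.
; Each requirement shows either a specific food name or "Any" plus the food type.
; A cast to the player character exists but is unconnected, so the overlapping actor is not filtered.
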(event `self.ReceiveActorBeginOverlap`
  (params (OtherActor :type "Actor Object Reference"))
  ;[1 1 1] Show Orders from Each Table
  (bind _outactors (`GameplayStatics.GetAllActorsOfClass` "/Game/Blueprints/JamesWen/SM_Prop_Table_4_Blueprint.SM_Prop_Table_4_Blueprint_C"))
  (for _array_element _outactors
    (`KismetSystemLibrary.PrintString` (`KismetStringLibrary.Concat_StrStr` "Table " (`KismetStringLibrary.Conv_IntToString` (`/Game/Blueprints/JamesWen/SM_Prop_Table_4_Blueprint.TableNumber` _array_element))))
    (for _array_element_2 (`/Game/Blueprints/JamesWen/SM_Prop_Table_4_Blueprint.OrderRequirements` _array_element)
      (bind (_requiredfoodname _requiredfoodtype _isspecificitem) (break `/Game/Blueprints/OrderRequirementStruct` _array_element_2))
      (if _isspecificitem
        (`KismetSystemLibrary.PrintString` (`KismetStringLibrary.Concat_StrStr` "Required: " _requiredfoodname))
        (else
          (`KismetSystemLibrary.PrintString` (`KismetStringLibrary.Concat_StrStr` "Required: Any " (`|GetEnumeratorNameAsString` _requiredfoodtype))))))))

(fn `UserConstructionScript`)