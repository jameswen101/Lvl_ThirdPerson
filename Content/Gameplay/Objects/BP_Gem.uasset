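; Collectible gem whose colour sets its mesh, material and value, with a GUID so already-collected gems destroy themselves on BeginPlay.
; Player overlap flies it along a cubic Bezier to the player, then increments the level gem count, spawns burst and floating-number feedback, and destroys it.
; A randomised timer plays a sparkle when the gem is distant, on screen and unobstructed.
; A separate timeline event animates it bursting out of a chest.
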(event `self.ReceiveBeginPlay`
  ;[1 1 1] Set the timer for the sparkle dinstance check
  (`self.DistanceSparkleTimer`)
  (if (`/Game/Gameplay/Modes/BP_SparkGameInstance.IsItemCollected` (`/Game/Gameplay/Modes/BPFL_SparkGameModes.GetSparkGameInstance`) "NewEnumerator1" (`self.GemGUID`))
    (`self.K2_DestroyActor`)))

(event `self.GemCollision.OnComponentBeginOverlap`
  (params (OverlappedComponent :type "PrimitiveComponent Object Reference") (OtherActor :type "Actor Object Reference") (OtherComp :type "PrimitiveComponent Object Reference") (OtherBodyIndex :type Integer) (bFromSweep :type Boolean) (SweepResult :type "HitResult Structure (by ref)"))
  (bind _returnvalue (`GameplayStatics.GetPlayerCharacter` 0))
  ;[1 1 1] When the player picks up the gem
  (cast `/Game/Gameplay/Characters/Player/BP_SparkCharacter_Player` OtherActor)
  (`/Engine/EditorBlueprintResources/StandardMacros.DoOnce` false
    (:`Completed`
      ;[1 1 1] Stop the explode timeline if we pick it up
      (`TimelineComponent.Stop` (`self.ExplodeFromChestTimeline`))
      ;[1 1 1] Detach the mesh, spawn the system and store the location
      (`GameplayStatics.PlaySoundAtLocation` "/Game/Objects/Gem/Sound/SC_GemPickedUpStart.SC_GemPickedUpStart" (`self.K2_GetActorLocation`) (struct) 1.0 1.0 0.0 null null null null)
      (bind _returnvalue_2 (`NiagaraFunctionLibrary.SpawnSystemAttached` "/Game/Objects/Gem/FX/FX_GemPickedUp_System.FX_GemPickedUp_System" (`self.GemMesh`) "None" (0.0 0.0 0.0) (struct) "KeepRelativeOffset" true))
      (bind _output_get (set `self.PickedUpParticleSystem` _returnvalue_2))
      (`NiagaraComponent.SetVariableLinearColor` _output_get "User.GemColour" (`/Game/Gameplay/Objects/BPFL_Gems.GetGemParticleColour` (`self.GemColour`)))
      (`SceneComponent.K2_DetachFromComponent` (`self.GemMeshRoot`) "KeepWorld" "KeepRelative" "KeepWorld" true)
      (set `self.StartPos` (`SceneComponent.K2_GetComponentLocation` (`self.GemMeshRoot`)))
      ;[1 1 1] Cubic bezier animation that translates to the player
      (bind (_direction _scale3d) (`Timeline|GemPickupTimeline`)
        (:`Update`
          (set `self.CumalativeDelta` (+ (`self.CumalativeDelta`) (`GameplayStatics.GetWorldDeltaSeconds`)))
          (`SceneComponent.SetRelativeScale3D` (`self.GemMesh`) (`KismetMathLibrary.Conv_DoubleToVector` _scale3d))
          (`SceneComponent.K2_SetWorldLocation` (`self.GemMeshRoot`) (`/Game/Gameplay/Curves/BPFL_Curves.CubicBezierCurve` (`self.CumalativeDelta`) (`self.StartPos`) (+ (/ (+ (`self.K2_GetActorLocation` (`GameplayStatics.GetPlayerCharacter` 0)) (`self.StartPos`)) 2.0) (0.0 0.0 150.0)) (+ (`self.StartPos`) (0.0 0.0 200.0)) (`self.K2_GetActorLocation` (`GameplayStatics.GetPlayerCharacter` 0))) false false))
        (:`Finished`
          ;[1 1 1] Signal that we've picked up a gem
          (`/Game/Gameplay/Modes/BP_SparkGameState.IncrementCurrentLevelGemCount` (`/Game/Gameplay/Modes/BPFL_SparkGameModes.GetSparkGameState`) (`self.GemValue`) (`self.GemGUID`))
          (`self.OnGemPickedUp` (`self.GemColour`) (`self.GemValue`))
          (`|ExecutionSequence`
            (:`then_0`
              ;[1 1 1] Spawn the final burst particle system
              (`GameplayStatics.PlaySoundAtLocation` "/Game/Objects/Gem/Sound/SC_GemPickedUpComplete.SC_GemPickedUpComplete" (`self.K2_GetActorLocation`) (struct) 1.0 1.0 0.0 null null null null)
              (bind _returnvalue_3 (`NiagaraFunctionLibrary.SpawnSystemAtLocation` "/Game/Objects/Gem/FX/FX_GemPickedUp_FinalBurst_System.FX_GemPickedUp_FinalBurst_System" (`self.K2_GetActorLocation` (`GameplayStatics.GetPlayerCharacter` 0))))
              (`NiagaraComponent.SetVariableVec3` _returnvalue_3 "User.PlayerVelocity" (`self.GetVelocity` (`GameplayStatics.GetPlayerCharacter` 0)))
              (`NiagaraComponent.SetVariableLinearColor` _returnvalue_3 "User.GemColour" (`/Game/Gameplay/Objects/BPFL_Gems.GetGemParticleColour` (`self.GemColour`)))
              ;[1 1 1] Spawn the bouncing number text actor
              (`|SpawnActorFromClass` "/Game/Gameplay/Objects/BP_GemFloatingNumber.BP_GemFloatingNumber_C" (`self.GetTransform` _returnvalue) "AlwaysSpawn" "OverrideRootScale" self (`KismetMathLibrary.GetForwardVector` (`KismetMathLibrary.FindLookAtRotation` (`self.K2_GetActorLocation` _returnvalue) (`self.K2_GetActorLocation`))) (`self.GemColour`) _returnvalue))
            (:`then_1`
              ;[1 1 1] Deactivate the particle system then destroy the actor
              (`ActorComponent.Deactivate` (`self.PickedUpParticleSystem`))
              (`KismetSystemLibrary.Delay` 2.0)
              (`self.K2_DestroyActor`))))))))

(event `DistanceSparkleTimer`
  (bind _returnvalue (`GameplayStatics.GetPlayerCharacter` 0))
  ;[1 1 1] Kick off the looping timer
  (`|ExecutionSequence`
    (:`then_0`
      (`/Engine/EditorBlueprintResources/StandardMacros.DoOnce` false
        (:`Completed`
          (`KismetSystemLibrary.K2_SetTimerDelegate` (delegate `DistanceSparkleTimer`) (`KismetMathLibrary.RandomFloatInRange` (`self.SparkleMinDelay`) (`self.SparkleMaxDelay`)) true))))
    (:`then_1`
      ;[1 1 1] Ensure the player is far enough away
      (`/Engine/EditorBlueprintResources/StandardMacros.IsValid` _returnvalue
        (:`Is Valid`
          (if (> (`self.GetDistanceTo` _returnvalue self) (`self.SparkMinimumDistance`))
            ;[1 1 1] Ensure that we can see the gem
            (if (`.ReturnValue` (`GameplayStatics.ProjectWorldToScreen` (`GameplayStatics.GetPlayerController` 0) (`self.K2_GetActorLocation`)))
              ;[1 1 1] Ensure that we have line of sight to the gem
              (bind (_outhit _returnvalue_2) (`KismetSystemLibrary.LineTraceSingle` (`PlayerCameraManager.GetCameraLocation` (`GameplayStatics.GetPlayerCameraManager` 0)) (`self.K2_GetActorLocation`) "TraceTypeQuery2" false (`|MakeArray` (`GameplayStatics.GetPlayerCharacter` 0) :!type "Actor Object Reference") "None" true (struct :`R` 0.183154 :`G` 1.0 :`A` 1.0) (struct :`R` 1.0 :`B` 0.139955 :`A` 1.0)))
              (if (not _returnvalue_2)
                (`NiagaraFunctionLibrary.SpawnSystemAttached` "/Game/Objects/Gem/FX/FX_GemDistanceSparkle_System.FX_GemDistanceSparkle_System" (`self.GemMesh`) "SparkleSocket" (0.0 0.0 0.0) (struct) "SnapToTarget" true)))))))))

(event `PlayExplodeFromSourceAnimation`
  (params (ChestLocation :type "Vector Structure"))
  ;[1 1 1] Explode from chest animation
  (`KismetSystemLibrary.Delay` (`KismetMathLibrary.RandomFloatInRange` 0.0 0.25))
  (bind (_direction _alpha _height) (`Timeline|ExplodeFromChestTimeline` :!via `PlayFromStart`)
    (:`Update`
      (`SceneComponent.K2_SetWorldLocation` (`self.GemMeshRoot`) (`KismetMathLibrary.VLerp` (+ ChestLocation (`KismetMathLibrary.MakeVector` 0.0 0.0 _height)) (+ (`SceneComponent.K2_GetComponentLocation` (`self.Scene`)) (`KismetMathLibrary.MakeVector` 0.0 0.0 _height)) _alpha) false false))))

(fn `GetGemValue`
  (returns (GemValue :type Integer))
  (return (`self.GemValue`)))

(fn `UserConstructionScript`
  (bind _gemidleanimationspeed (`self.GemIdleAnimationSpeed`))
  (bind (_gemvalue _gemstaticmesh _gemmaterial) (`/Game/Gameplay/Objects/BPFL_Gems.GetGemData` (`self.GemColour`)))
  ;[1 1 1] Set how fast it takes the gem to idle animate
  (`TimelineComponent.SetPlaybackPosition` (`self.GemIdleTimeline`) (`KismetMathLibrary.RandomFloatInRange` 0.0 1.0) false true)
  (`TimelineComponent.SetPlayRate` (`self.GemIdleTimeline`) (/ 1.0 (`KismetMathLibrary.RandomFloatInRange` (- _gemidleanimationspeed (* _gemidleanimationspeed 0.1)) (+ _gemidleanimationspeed (* _gemidleanimationspeed 0.1)))))
  ;[1 1 1] Set the gem to red if someone is trying to be sneaky and set it to none
  (if (`|EnumEquality` (`self.GemColour`) "NewEnumerator0")
    (set `self.GemColour` "NewEnumerator1"))
  ;[1 1 1] Initialize the gem based on it's colour
  (set `self.GemValue` _gemvalue)
  (`StaticMeshComponent.SetStaticMesh` (`self.GemMesh`) _gemstaticmesh)
  (`PrimitiveComponent.SetMaterial` (`self.GemMesh`) 0 _gemmaterial)
  ;[1 1 1] Generate a unique GUID for the gem
  (if (not (`KismetGuidLibrary.IsValid_Guid` (`self.GemGUID`)))
    (set `self.GemGUID` (`KismetGuidLibrary.NewGuid`)))
  (`SphereComponent.SetSphereRadius` (`self.GemCollision`) (`self.GemRange`) true))