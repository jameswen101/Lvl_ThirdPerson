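; BP_GemFloatingNumber is a short-lived actor that shows a gem's value as a bouncing number popup.
; On BeginPlay it sets the widget text from the gem colour and launches a physics sphere with a forward and upward impulse.
; Hand-tuned delays, matched to the widget animation and physics, then play a disappear sound, shrink the text, spawn a burst effect and destroy the actor.
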(event `self.ReceiveBeginPlay`
  (bind (_returnvalue_x _returnvalue_y) (`KismetMathLibrary.BreakVector` (* (`self.ForwardVector`) (`self.XYImpulse`))))
  ;[1 1 1] Set the number in the widget acording to the gem's value
  (bind _output_get (set `self.FloatingNumberWidget` (cast `/Game/UI/Widgets/InGame/WBP_GemBouncingText` (`WidgetComponent.GetUserWidgetObject` (`self.NumberWidget`)) :!pure true)))
  (`/Game/UI/Widgets/InGame/WBP_GemBouncingText.SetGemValueText` _output_get (`self.GemColour`))
  ;[1 1 1] Add an impulse to the bouncing physics object
  (`PrimitiveComponent.AddImpulse` (`self.BouncySphere`) (`KismetMathLibrary.MakeVector` _returnvalue_x _returnvalue_y (`self.ZImpulse`)) "None" false)
  ;[1 1 1] Timing hacks due to widget animations and physics simulation
  (`KismetSystemLibrary.Delay` 0.85) ; 1.425 total time
  ;;[1 1 1] Play the SFX
  (`GameplayStatics.PlaySoundAtLocation` "/Game/Objects/Gem/Sound/SC_GemFloatingNumberDisappear.SC_GemFloatingNumberDisappear" (`self.K2_GetActorLocation`) (struct) 1.0 1.0 0.0 null null null null)
  (`KismetSystemLibrary.Delay` 0.40838)
  (`/Game/UI/Widgets/InGame/WBP_GemBouncingText.PlayGemTextShrinkAnimation` (`self.FloatingNumberWidget`))
  (`KismetSystemLibrary.Delay` 0.16)
  ;[1 1 1] Spawn the FX
  (`NiagaraFunctionLibrary.SpawnSystemAtLocation` "/Game/Objects/Gem/FX/FX_GemNumberBurst_System.FX_GemNumberBurst_System" (`SceneComponent.K2_GetComponentLocation` (`self.NumberWidget`)))
  ;[1 1 1] Destroy the actor
  (`self.K2_DestroyActor`))

(fn `UserConstructionScript`)