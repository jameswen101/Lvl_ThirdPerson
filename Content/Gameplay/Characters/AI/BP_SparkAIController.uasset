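; AI controller for Spark AI characters that runs their behavior trees and targets the player through perception.
; On possess, it runs the character's base tree, injects its combat, idle and leash subtrees by gameplay tag, and records the first spawn location as LeashOrigin.
; Sensing a Player-tagged actor sets the blackboard Target.
; Losing sight clears it after a gated delay if CanLoseTarget allows, unless the player is sensed again.
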(event `self.AIPerception.OnTargetPerceptionUpdated`
  (params (Actor :type "Actor Object Reference") (Stimulus :type "AIStimulus Structure"))
  ;[1 1 1] Setting the player as the target
  (`/Engine/EditorBlueprintResources/StandardMacros.IsValid` Actor
    (:`Is Valid`
      (if (`KismetArrayLibrary.Array_Contains` (`Actor.Tags` Actor) "Player")
        (if (`.bSuccessfullySensed` (break `AIStimulus` Stimulus))
          (`BlackboardComponent.SetValueAsObject` (`self.Blackboard`) "Target" Actor)
          (goto _label :!via `Close`)
          (else
            (`|ExecutionSequence`
              (:`then_0`
                (goto _label :!via `Open`))
              (:`then_1`
                (`KismetSystemLibrary.Delay` 3.0)
                (`/Engine/EditorBlueprintResources/StandardMacros.Gate` false :!label _label
                  (:`Exit`
                    (if (`self.CanLoseTarget`) :!label _label_2
                      (`BlackboardComponent.SetValueAsObject` (`self.Blackboard`) "Target" null))))))))))
    (:`Is Not Valid`
      (goto _label_2))))

(event `self.ReceivePossess`
  (params (PossessedPawn :type "Pawn Object Reference"))
  ;[1 1 1] Give the AI it's proper behaviour trees from it's class
  (bind _asbp_spark_character_ai (cast `/Game/Gameplay/Characters/AI/BP_SparkCharacter_AI` PossessedPawn))
  (`self.RunBehaviorTree` (`/Game/Gameplay/Characters/AI/BP_SparkCharacter_AI.BaseTree` _asbp_spark_character_ai))
  (bind _asbehavior_tree_component (cast `BehaviorTreeComponent` (`self.BrainComponent`)))
  (`BehaviorTreeComponent.SetDynamicSubtree` _asbehavior_tree_component (struct :`TagName` "AI.CombatSubtree") (`/Game/Gameplay/Characters/AI/BP_SparkCharacter_AI.CombatSubtree` _asbp_spark_character_ai))
  (`BehaviorTreeComponent.SetDynamicSubtree` _asbehavior_tree_component (struct :`TagName` "AI.IdleSubtree") (`/Game/Gameplay/Characters/AI/BP_SparkCharacter_AI.IdleSubtree` _asbp_spark_character_ai))
  (`BehaviorTreeComponent.SetDynamicSubtree` _asbehavior_tree_component (struct :`TagName` "AI.LeashSubtree") (`/Game/Gameplay/Characters/AI/BP_SparkCharacter_AI.LeashSubtree` _asbp_spark_character_ai))
  (set `self.CanLoseTarget` (`/Game/Gameplay/Characters/AI/BP_SparkCharacter_AI.CanLoseTarget` _asbp_spark_character_ai))
  (`/Engine/EditorBlueprintResources/StandardMacros.DoOnce` false
    (:`Completed`
      (`BlackboardComponent.SetValueAsVector` (`self.Blackboard`) "LeashOrigin" (`self.K2_GetActorLocation` (`self.K2_GetPawn`))))))

(event `self.BrainComponent.OnComponentActivated`
  (params (Component :type "ActorComponent Object Reference") (bReset :type Boolean))
  (`KismetSystemLibrary.PrintString` "Hello"))

(event `self.ReceiveBeginPlay`)

(fn `UserConstructionScript`)