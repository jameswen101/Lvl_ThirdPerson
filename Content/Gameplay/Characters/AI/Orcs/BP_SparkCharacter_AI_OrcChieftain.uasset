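; Orc Chieftain AI character with a ground slam, an axe whirlwind and an enrage state.
; Slam spawns an AoE actor ahead; whirlwind sphere-traces from the axe hand, using DoOnce to limit player damage per call.
; Damage while calm triggers enrage, which ignores further damage until ended.
; Enrage fades skin colour via timeline and dynamic material, briefly unpossesses the AI, then sets its Blackboard flag.
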(event `ChieftainSlam`
  (bind (_returnvalue_location _returnvalue_rotation _returnvalue_scale) (`KismetMathLibrary.BreakTransform` (`self.GetTransform`)))
  ;[1 1 1] Ground slam
  (`|SpawnActorFromClass` "/Game/Gameplay/Combat/BP_AoEAttack_ChieftainSlam.BP_AoEAttack_ChieftainSlam_C" (`KismetMathLibrary.MakeTransform` (+ (* (`self.GetActorForwardVector`) 200.0) _returnvalue_location) _returnvalue_rotation _returnvalue_scale) "Undefined" "OverrideRootScale" self (`self.GetInstigator`)))

(event `self.ReceiveAnyDamage`
  (params (Damage :type "Float (single-precision)") (DamageType :type "DamageType Object Reference") (InstigatedBy :type "Controller Object Reference") (DamageCauser :type "Actor Object Reference"))
  ;[1 1 1] Modify damage taken based on enrage
  (if (not (`self.IsEnraged`))
    (`parent.ReceiveAnyDamage` Damage DamageType InstigatedBy DamageCauser)
    (`self.StartEnrage`)))

(event `ChieftainWhirlwind`
  (bind _returnvalue (`SceneComponent.GetSocketLocation` (`self.Mesh`) "RightHandSocket"))
  ;[1 1 1] Whirlwind
  (bind _outhits (`KismetSystemLibrary.SphereTraceMultiForObjects` _returnvalue (+ _returnvalue (* (`self.GetActorForwardVector`) 100.0)) 120.0 (`|MakeArray` "ObjectTypeQuery3" :!type "EObjectTypeQuery Enum")))
  (`|ExecutionSequence`
    (:`then_0`
      (goto _label :!via `Reset`))
    (:`then_1`
      (for _array_element _outhits
        (`/Engine/EditorBlueprintResources/StandardMacros.DoOnce` false :!label _label
          (:`Completed`
            (bind _asbp_spark_character_player (cast `/Game/Gameplay/Characters/Player/BP_SparkCharacter_Player` (`.HitActor` (`GameplayStatics.BreakHitResult` _array_element))))
            (`GameplayStatics.ApplyDamage` _asbp_spark_character_player 2.0 (`self.GetController`) self "/Game/Gameplay/Logic/DamageTypes/DT_Piercing.DT_Piercing_C")))))))

(event `StartEnrage`
  (bind _returnvalue (`AIBlueprintHelperLibrary.GetAIController` self))
  ;[1 1 1] Start enrage
  (set `self.IsEnraged` true)
  (`self.StartEnrageSkinTone`)
  (set `self.AIControllerReference` _returnvalue)
  (`Controller.UnPossess` _returnvalue)
  (`KismetSystemLibrary.Delay` 2.69)
  (`Controller.Possess` (`self.AIControllerReference`) self)
  (`BlackboardComponent.SetValueAsBool` (`AIController.Blackboard` (`self.AIControllerReference`)) "IsEnraged" true))

(event `EndEnrage`
  ;[1 1 1] End enrage
  (set `self.IsEnraged` false)
  (`self.ReverseEnrageSkinTone`))

(event `StartEnrageSkinTone`
  ;[1 1 1] Enrage - Lerp the skin color
  (bind (_direction _alpha) (`Timeline|EnrageSkinToneChange` :!via `PlayFromStart` :!label _label_2)
    (:`Update`
      (`MaterialInstanceDynamic.SetScalarParameterValue` (`self.ChieftainDMI`) "SkinColourAlpha" _alpha))))

(event `ReverseEnrageSkinTone`
  ;[1 1 1] Enrage - Lerp the skin color
  (goto _label_2 :!via `ReverseFromEnd`))

(fn `UserConstructionScript`
  (`parent.UserConstructionScript`)
  (`SceneComponent.K2_AttachToComponent` (`self.ChieftanAxe`) (`self.Mesh`) "RightHandSocket" "SnapToTarget" "KeepRelative" "KeepRelative" true)
  (bind _returnvalue (`PrimitiveComponent.CreateDynamicMaterialInstance` (`self.Mesh`) 0 "/Game/Characters/OrcChieftain/Materials/Mat_OrcChieftain_Inst.Mat_OrcChieftain_Inst" "None"))
  (set `self.ChieftainDMI` _returnvalue))