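; Base Spark character that manages health, damage-type immunities, hit reactions and death, broadcasting health changes through Call functions.
; AnyDamage skips immune types, heals on non-positive amounts, and otherwise applies damage only if CanTakeDamage is set and no stun is active.
; Non-lethal hits play a montage, timed stun and FX; death plays an animation, ignores Pawn collision, then runs delayed FX and destruction.
; Controller-input hooks are empty, and SetCurrentHealth broadcasts without storing.
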(event `self.ReceiveAnyDamage`
  (params (Damage :type "Float (single-precision)") (DamageType :type "DamageType Object Reference") (InstigatedBy :type "Controller Object Reference") (DamageCauser :type "Actor Object Reference"))
  ;[1 1 1] Only damage them if they are not damage immune
  (if (not (`self.GetIsDamageTypeImmune` (`GameplayStatics.GetObjectClass` DamageType)))
    (if (> Damage 0.0)
      ;[1 1 1] used for debug
      (if (`self.CanTakeDamage`)
        (`self.DamageStunned`
          (:`false`
            (bind _isdead (`self.DamageCharacter` Damage))
            (if _isdead
              (`/Engine/EditorBlueprintResources/StandardMacros.DoOnce` false
                (:`Completed`
                  (`self.KillCharacter`)
                  (`KismetSystemLibrary.Delay` (`self.DelayBeforeDeathFX`))
                  (`self.PlayDestroyedFX`)
                  (`self.StartDestroyCountdown`)))))))
      (else
        (`self.HealCharacter` (* Damage -1.0))))))

(event `StartDestroyCountdown`
  (`KismetSystemLibrary.Delay` 2.0)
  (`self.CleanUpDeadCharacter`))

(event `ApplyHealing`
  (params (BaseHealing :type "Float (double-precision)") (`Instigated By` :type "Controller Object Reference") (`Heal Causer` :type "Actor Object Reference") (`Heal Type` :type "DamageType Class Reference"))
  (`self.HealCharacter` BaseHealing))

(fn `AddDamageTypeImmunity`
  (params (NewItem :type "DamageType Class Reference"))
  (returns (Return :type Boolean))
  (`BlueprintSetLibrary.Set_Add` (`self.DamageImmunities`) NewItem)
  (return true))

(fn `CleanUpDeadCharacter`
  (`self.K2_DestroyActor`))

(fn `DamageCharacter`
  (params (Damage :type "Float (double-precision)"))
  (returns (IsDead :type Boolean))
  (locals (LocalDamage :type "Float (double-precision)") (LocalIsDead :type Boolean :default false))
  (bind _output_get (set `local.LocalDamage` Damage))
  (bind _newhealth (`self.ModifyHealth` _output_get "NewEnumerator1"))
  (set `local.LocalIsDead` (not (> _newhealth 0)))
  (`self.OnCharacterDamaged` self (`local.LocalDamage`) _newhealth (`local.LocalIsDead`))
  (if (not (`local.LocalIsDead`))
    (`/Engine/EditorBlueprintResources/StandardMacros.IsValid` (`self.DamagedAnimation`)
      (:`Is Valid`
        (`self.DamagedStunBegin`)
        (`KismetSystemLibrary.K2_SetTimer` null "DamagedStunEnd" (`AnimSequenceBase.GetPlayLength` (`self.DamagedAnimation`)))
        (`AnimInstance.Montage_Play` (`SkeletalMeshComponent.GetAnimInstance` (`self.Mesh`)) (`self.DamagedAnimation`) 1.0 "MontageLength" 0.0 true)
        (`self.PlayDamagedFX`)
        (return (`local.LocalIsDead`)))
      (:`Is Not Valid`
        _)))
  (return (`local.LocalIsDead`)))

(fn `DamagedStunBegin`
  (set `self.IsDamagedStunned` true))

(fn `DamagedStunEnd`
  (set `self.IsDamagedStunned` false))

(fn `DisableCharacterControllerInput`)

(fn `EnableCharacterControllerInput`)

(fn `GetAllDamageTypeImmunities`
  (returns (DamageImmunities :type "Set of DamageType Class Reference"))
  (return (`self.DamageImmunities`)))

(fn `GetCurrentHealth`
  (returns (CurrentHealth :type Integer))
  (return (`self.CurrentHealth`)))

(fn `GetIsAlive`
  (returns (ReturnValue :type Boolean))
  (return (> (`self.CurrentHealth`) 0)))

(fn `GetIsDamageTypeImmune`
  (params (DamageType :type "DamageType Class Reference (by ref)"))
  (returns (IsImmune :type Boolean))
  (return (`BlueprintSetLibrary.Set_Contains` (`self.DamageImmunities`) DamageType)))

(fn `GetMaxHealth`
  (returns (MaxHealth :type Integer))
  (return (`self.MaxHealth`)))

(fn `HealCharacter`
  (params (HealAmount :type "Float (double-precision)"))
  (bind _newhealth (`self.ModifyHealth` HealAmount))
  (`self.OnCharacterHealed` self HealAmount _newhealth))

(fn `IsAtMaxHealth`
  (returns (ReturnValue :type Boolean))
  (return (== (`self.CurrentHealth`) (`self.MaxHealth`))))

(fn `KillCharacter`
  (`self.DisableCharacterControllerInput`)
  (`SkeletalMeshComponent.PlayAnimation` (`self.Mesh`) (`self.DeathAnimation`) false)
  (`PrimitiveComponent.SetCollisionResponseToChannel` (`self.CapsuleComponent`) "ECC_Pawn" "ECR_Ignore")
  (`self.OnCharacterDead` self))

(fn `ModifyHealth`
  (params (Amount :type "Float (double-precision)") (ModifyMeothd :type "/Game/Gameplay/Characters/Player/Enums/EHealthModifyMethod Enum" :default "NewEnumerator0"))
  (returns (NewHealth :type Integer))
  (bind _output_get (set `self.CurrentHealth` (`KismetMathLibrary.Clamp` (select `/Game/Gameplay/Characters/Player/Enums/EHealthModifyMethod` ModifyMeothd :`NewEnumerator0` (+ (`self.CurrentHealth`) (`KismetMathLibrary.FTrunc` Amount)) :`NewEnumerator1` (- (`self.CurrentHealth`) (`KismetMathLibrary.FTrunc` Amount))) 0 (`self.MaxHealth`))))
  (`self.OnCharacterHealthModified` self _output_get)
  (return _output_get))

(fn `PlayDamagedFX`
  (bind (_returnvalue_location _returnvalue_rotation _returnvalue_scale) (`KismetMathLibrary.BreakTransform` (`self.GetTransform`)))
  (`NiagaraFunctionLibrary.SpawnSystemAtLocation` (`self.DamagedVFX`) _returnvalue_location _returnvalue_rotation _returnvalue_scale)
  (`GameplayStatics.PlaySoundAtLocation` (`self.DamagedSFX`) (`self.K2_GetActorLocation`) (struct) 1.0 1.0 0.0 null null null null))

(fn `PlayDestroyedFX`
  (returns (VFXSystem :type "NiagaraComponent Object Reference"))
  (bind _mesh (`self.Mesh`))
  (bind _returnvalue (`NiagaraFunctionLibrary.SpawnSystemAttached` (`self.DestroyVFX`) _mesh (`.ReturnValue` (`SkinnedMeshComponent.FindClosestBone_K2` _mesh (`PrimitiveComponent.GetCenterOfMass` _mesh "None") 0.0 false)) (0.0 0.0 0.0) (struct) "SnapToTargetIncludingScale" false true "AutoRelease"))
  (`GameplayStatics.PlaySoundAtLocation` (`self.DestroySFX`) (`self.K2_GetActorLocation`) (struct) 1.0 1.0 0.0 null null null null)
  (return _returnvalue))

(fn `Remove Damage Type Immunity`
  (params (Item :type "DamageType Class Reference"))
  (returns (ReturnValue :type Boolean))
  (bind _returnvalue (`BlueprintSetLibrary.Set_Remove` (`self.DamageImmunities`) Item))
  (return _returnvalue))

(fn `SetCurrentHealth`
  (params (Health :type "Float (double-precision)"))
  (returns (NewHealth :type Integer))
  (bind _returnvalue (`KismetMathLibrary.Clamp` (`KismetMathLibrary.FTrunc` Health) 0 (`self.MaxHealth`)))
  (`self.OnCharacterHealthModified` self _returnvalue)
  (return _returnvalue))

(fn `UserConstructionScript`
  (set `self.CurrentHealth` (`self.MaxHealth`)))