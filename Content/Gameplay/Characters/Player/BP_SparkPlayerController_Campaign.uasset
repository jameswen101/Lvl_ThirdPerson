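; Campaign player controller that handles pausing and the guidebook from the Pause and Guidebook inputs.
; Pause pops the top Spark HUD widget, resuming play if it was the pause menu or guidebook, and opens the pause menu when nothing pops.
; The guidebook toggles through the HUD, sharing its close path with Pause.
; Two helper events switch game pause, input mode and mouse cursor together.
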(event `SetControllerToPlay`
  ;[1 1 1] Comment
  (`GameplayStatics.SetGamePaused` false)
  (`WidgetBlueprintLibrary.SetInputMode_GameOnly` self)
  (set `self.bShowMouseCursor` false))

(event `SetControllerToPause`
  ;[1 1 1] Comment
  (`GameplayStatics.SetGamePaused` true)
  (`WidgetBlueprintLibrary.SetInputMode_GameAndUIEx` self null)
  (set `self.bShowMouseCursor` true))

(event `InputAction|Pause` :paused true
  (params (Key :type "Key Structure"))
  ;[1 1 1] Pause
  (:`Pressed`
    (`self.TogglePauseGame`)))

(event `self.TogglePauseGame`
  ;[1 1 1] Pause
  (bind (_widgetpopped _poppedwidget) (`/Game/Gameplay/Characters/Player/BP_SparkHUD.PopWidget` (`/Game/Gameplay/Modes/BPFL_SparkGameModes.GetSparkHUD`)))
  (if _widgetpopped
    (bind _returnvalue (`GameplayStatics.GetObjectClass` _poppedwidget))
    (if (== _returnvalue "/Game/UI/Widgets/Menus/WBP_PauseMenu.WBP_PauseMenu_C")
      (set `self.IsPauseMenuOpen` false)
      (`self.SetControllerToPlay`)
      (elif (== _returnvalue "/Game/UI/Widgets/Menus/WBP_Guidebook.WBP_Guidebook_C")
        ;[1 1 1] Guidebook
        (set `self.IsGuidebookOpen` false :!label _label)
        (`/Game/Gameplay/Characters/Player/BP_SparkHUD.SetEnableGuidebook` (`/Game/Gameplay/Modes/BPFL_SparkGameModes.GetSparkHUD`) false)
        (`self.SetControllerToPlay`)))
    (else
      (set `self.IsPauseMenuOpen` true)
      (`/Game/Gameplay/Characters/Player/BP_SparkHUD.SetEnablePause Menu` (`/Game/Gameplay/Modes/BPFL_SparkGameModes.GetSparkHUD`) true)
      (`self.SetControllerToPause`))))

(event `ToggleGuidebook`
  ;[1 1 1] Guidebook
  (if (`self.IsGuidebookOpen`)
    (goto _label)
    (else
      (set `self.IsGuidebookOpen` true)
      (`/Game/Gameplay/Characters/Player/BP_SparkHUD.SetEnableGuidebook` (`/Game/Gameplay/Modes/BPFL_SparkGameModes.GetSparkHUD`) true)
      (`self.SetControllerToPause`))))

(event `InputAction|Guidebook` :paused true
  (params (Key :type "Key Structure"))
  ;[1 1 1] Guidebook
  (:`Pressed`
    (`self.ToggleGuidebook`)))

(fn `UserConstructionScript`
  (`parent.UserConstructionScript`))