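; BP_SparkHUD_Campaign is the campaign HUD Blueprint that creates the player's main UI widgets.
; On BeginPlay it runs the parent logic, then calls one custom event each for the player HUD, guidebook and pause menu, storing each widget in a variable.
; Only the player HUD is added to the viewport; the guidebook and pause menu are created up front without being displayed here.
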(event `self.ReceiveBeginPlay`
  (`parent.ReceiveBeginPlay`)
  (`self.CreatePlayerHUDWidget`)
  (`self.CreateGuidebookWidget`)
  (`self.CreatePauseMenuWidget`))

(event `CreatePlayerHUDWidget`
  ;[1 1 1] Create the HUD
  (bind _returnvalue (`|CreateWidget` "/Game/UI/Widgets/HUD/WBP_PlayerHUD.WBP_PlayerHUD_C"))
  (bind _output_get (set `self.HUDWidget` _returnvalue))
  (`UserWidget.AddToViewport` _output_get 0))

(event `CreateGuidebookWidget`
  ;[1 1 1] Create the guidebook
  (bind _returnvalue (`|CreateWidget` "/Game/UI/Widgets/Menus/WBP_Guidebook.WBP_Guidebook_C"))
  (set `self.GuidebookWidget` _returnvalue))

(event `CreatePauseMenuWidget`
  ;[1 1 1] Create the pause menu
  (bind _returnvalue (`|CreateWidget` "/Game/UI/Widgets/Menus/WBP_PauseMenu.WBP_PauseMenu_C"))
  (set `self.PauseMenuWidget` _returnvalue))

(fn `UserConstructionScript`
  (`parent.UserConstructionScript`))