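; Projectile actor that ignores its instigator and deals piercing damage to the first Character it overlaps.
; A multi-input DoOnce gates blocking hits and character overlaps into a shared stop and impact routine, with damage only on the overlap path.
; Impact shuts off trail effects and looping audio, spawns VFX and sound, then destroys the actor, optionally after sticking briefly and playing disappear effects.
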(event `self.ReceiveHit`
  (params (MyComp :type "PrimitiveComponent Object Reference") (Other :type "Actor Object Reference") (OtherComp :type "PrimitiveComponent Object Reference") (bSelfMoved :type Boolean) (HitLocation :type "Vector Structure") (HitNormal :type "Vector Structure") (NormalImpulse :type "Vector Structure") (Hit :type "HitResult Structure (by ref)"))
  ;[1 1 1] Comment
  ;[1 1 1] Comment
  (`|DoOnceMultiInput` :!label _label
    (:`A Out`
      _)
    (:`B Out`
      (`self.DamageOverlappingActor`)))
  (`self.StopProjectile`)
  (`self.PlayHitFX`))

(event `self.ReceiveBeginPlay`
  ;[1 1 1] Ignore the instigator
  (`PrimitiveComponent.IgnoreActorWhenMoving` (`self.ProjectileCollision`) (`self.GetInstigator`) true))

(event `PlayHitFX`
  ;[1 1 1] Turn off looping FX
  (`ActorComponent.Deactivate` (`self.VFXTrail`))
  (`AudioComponent.FadeOut` (`self.SFXLooping`) 0.2 0.0 "Linear")
  ;[1 1 1] Spawn impact
  (`NiagaraFunctionLibrary.SpawnSystemAtLocation` (`self.ProjectileImpactVFX`) (`self.K2_GetActorLocation`) (`self.K2_GetActorRotation`))
  (`GameplayStatics.SpawnSoundAtLocation` (`self.ProjectileImpactSFX`) (`self.K2_GetActorLocation`) (struct) 1.0 1.0 0.0 null null)
  ;[1 1 1] If we stick in the object, wait then play the disappear FX
  (if (`self.ProjectileStickInObject`)
    (`KismetSystemLibrary.Delay` (`self.ProjectileStickInObjectTime`))
    (`NiagaraFunctionLibrary.SpawnSystemAtLocation` (`self.ProjectileDisappearVFX`) (`self.K2_GetActorLocation`))
    (`GameplayStatics.SpawnSoundAtLocation` (`self.ProjectileDisappearSFX`) (`self.K2_GetActorLocation`) (struct) 1.0 1.0 0.0 null null)
    (`self.K2_DestroyActor`)
    (else
      (`self.K2_DestroyActor`))))

(event `StopProjectile`
  ;[1 1 1] Comment
  (`MovementComponent.StopMovementImmediately` (`self.ProjectileMovement`))
  (`ProjectileMovementComponent.StopSimulating` (`self.ProjectileMovement`) (`GameplayStatics.MakeHitResult` false)))

(event `self.ProjectileCollision.OnComponentBeginOverlap`
  (params (OverlappedComponent :type "PrimitiveComponent Object Reference") (OtherActor :type "Actor Object Reference") (OtherComp :type "PrimitiveComponent Object Reference") (OtherBodyIndex :type Integer) (bFromSweep :type Boolean) (SweepResult :type "HitResult Structure (by ref)"))
  ;[1 1 1] Comment
  (cast `Character` OtherActor)
  (goto _label :!via `B In`))

(event `DamageOverlappingActor`
  ;[1 1 1] Comment
  (`GameplayStatics.ApplyDamage` (stale `self.ProjectileCollision.OnComponentBeginOverlap` OtherActor) 1.0 (`self.GetInstigatorController`) self "/Game/Gameplay/Logic/DamageTypes/DT_Piercing.DT_Piercing_C"))

(fn `UserConstructionScript`)