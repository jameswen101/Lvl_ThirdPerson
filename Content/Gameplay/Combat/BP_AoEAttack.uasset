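; BP_AoEAttack is a ground-targeted area attack that telegraphs with a decal, then damages the player.
; On spawn it traces down, snaps to the ground and aligns to the surface normal.
; Timed startup, active and recovery phases swap VFX and sound, with damage applied once to an overlapping player as active begins.
; One decal timeline, rate-scaled to phase length, fades in during startup and reverses during recovery before delayed self-destruction.
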(event `self.ReceiveBeginPlay`
  ;[1 1 1] Begin play
  (`self.Startup`))

(event `Startup`
  (bind _returnvalue (`self.K2_GetActorLocation`))
  ;[1 1 1] Cast to the ground and align to angle
  (bind _outhit (`KismetSystemLibrary.LineTraceSingle` _returnvalue (- _returnvalue (0.0 0.0 5000.0)) "TraceTypeQuery2" false (`|MakeArray` (`GameplayStatics.GetPlayerCharacter` 0) :!type "Actor Object Reference")))
  (bind (_bblockinghit _binitialoverlap _time _distance _location _impactpoint _normal _impactnormal) (`GameplayStatics.BreakHitResult` _outhit))
  (`self.K2_SetActorLocationAndRotation` _impactpoint (`KismetMathLibrary.MakeRotFromZ` _impactnormal))
  ;[1 1 1] Play the decal
  (`TimelineComponent.SetPlayRate` (`self.DecalPowerIncreaseTimeline`) (/ 1.0 (+ (`self.StartupTime`) 0.01)))
  (`self.PlayDecalPowerIncrease`)
  (bind _returnvalue_2 (`GameplayStatics.SpawnSoundAtLocation` (`self.SFX_Startup`) (`self.K2_GetActorLocation`) (struct) 1.0 1.0 0.0 null null))
  (set `self.StartupSoundComponent` _returnvalue_2)
  ;[1 1 1] Delay then active
  (`KismetSystemLibrary.Delay` (`self.StartupTime`))
  (`self.Active`))

(event `TriggerAoEDamage`
  (bind _output (`|GetArrayItem` (`PrimitiveComponent.GetOverlappingActors` (`self.Capsule`) "/Game/Gameplay/Characters/Player/BP_SparkCharacter_Player.BP_SparkCharacter_Player_C")))
  ;[1 1 1] AoE damage functionality
  (`/Engine/EditorBlueprintResources/StandardMacros.IsValid` _output
    (:`Is Valid`
      (`GameplayStatics.ApplyDamage` _output (`self.BaseDamage`) (`self.GetInstigatorController`) self))))

(event `PlayDecalPowerIncrease`
  ;[1 1 1] VFX timeline
  (bind (_direction _alpha) (`Timeline|DecalPowerIncreaseTimeline` :!label _label)
    (:`Update`
      (`MaterialInstanceDynamic.SetScalarParameterValue` (`self.DecalMaterial`) "Power" (`KismetMathLibrary.Lerp` 1.0 500.0 _alpha))
      (`MaterialInstanceDynamic.SetScalarParameterValue` (`self.DecalMaterial`) "Opacity" (`KismetMathLibrary.Lerp` 0.0 1.0 _alpha)))
    (:`Finished`
      ;[1 1 1] Effect over
      (switch `ETimelineDirection` _direction
        (:`Backward`
          (`ActorComponent.Deactivate` (`self.VFX_Recovery`))
          ;[1 1 1] Cleanup
          (`KismetSystemLibrary.Delay` 4.0)
          (`self.K2_DestroyActor`))))))

(event `ReverseDecalPowerIncrease`
  ;[1 1 1] VFX timeline
  (goto _label :!via `Reverse`))

(event `Active`
  ;[1 1 1] Active
  (`GameplayStatics.PlaySoundAtLocation` (`self.SFX_Active`) (`self.K2_GetActorLocation`) (struct) 1.0 1.0 0.0 null null null null)
  (`ActorComponent.Deactivate` (`self.VFX_Startup`))
  (`ActorComponent.Activate` (`self.VFX_Active`) false)
  (`self.TriggerAoEDamage`)
  (`KismetSystemLibrary.Delay` (`self.ActiveTime`))
  (`self.Recovery`))

(event `Recovery`
  (bind _startupsoundcomponent (`self.StartupSoundComponent`))
  ;[1 1 1] Recovery
  (`GameplayStatics.PlaySoundAtLocation` (`self.SFX_Release`) (`self.K2_GetActorLocation`) (struct) 1.0 1.0 0.0 null null null null)
  (`/Engine/EditorBlueprintResources/StandardMacros.IsValid` _startupsoundcomponent
    (:`Is Valid`
      (`AudioComponent.FadeOut` _startupsoundcomponent (`self.RecoveryTime`) 0.0 "Linear"))
    (:`Is Not Valid`
      _))
  (`ActorComponent.Deactivate` (`self.VFX_Active`))
  (`ActorComponent.Activate` (`self.VFX_Recovery`) false)
  (`TimelineComponent.SetPlayRate` (`self.DecalPowerIncreaseTimeline`) (/ 1.0 (+ (`self.RecoveryTime`) 0.01)))
  (`self.ReverseDecalPowerIncrease`))

(fn `UserConstructionScript`
  ;[1 1 1] Create the dynamic material
  (bind _returnvalue (`DecalComponent.CreateDynamicMaterialInstance` (`self.Decal`)))
  (set `self.DecalMaterial` _returnvalue))