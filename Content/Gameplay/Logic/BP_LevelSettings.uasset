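; BP_LevelSettings holds a level's name, author and total gem and dragon egg counts.
; UpdateTotalCollectibleCounts recomputes the totals by scanning all actors of each collectible-related class.
; It sums gem values from placed gems, chest contents and BP_SparkCharacter_AI characters, and counts BP_DragonEgg actors for eggs.
; GetLevelSettings returns the four values together, while the construction script is empty.
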(fn `GetLevelSettings`
  (returns (LevelName :type Text) (AuthorName :type Text) (TotalGems :type Integer) (TotalEggs :type Integer))
  (return (`self.LevelName`) (`self.AuthorName`) (`self.TotalGems`) (`self.TotalEggs`)))

(fn `UpdateTotalCollectibleCounts`
  (set `self.TotalGems` 0)
  (set `self.TotalEggs` 0)
  (bind _outactors (`GameplayStatics.GetAllActorsOfClass` "/Game/Gameplay/Objects/BP_Gem.BP_Gem_C"))
  (for _array_element _outactors
    (set `self.TotalGems` (+ (`self.TotalGems`) (`/Game/Gameplay/Objects/BP_Gem.GetGemValue` _array_element))))
  (bind _outactors_2 (`GameplayStatics.GetAllActorsOfClass` "/Game/Gameplay/Objects/BP_Chest.BP_Chest_C"))
  (for _array_element_2 _outactors_2
    (set `self.TotalGems` (+ (`self.TotalGems`) (`/Game/Gameplay/Objects/BP_Chest.GetContainedTotalGemValue` _array_element_2))))
  (bind _outactors_3 (`GameplayStatics.GetAllActorsOfClass` "/Game/Gameplay/Characters/AI/BP_SparkCharacter_AI.BP_SparkCharacter_AI_C"))
  (for _array_element_3 _outactors_3
    (set `self.TotalGems` (+ (`self.TotalGems`) (`/Game/Gameplay/Characters/AI/BP_SparkCharacter_AI.GetTotalGemValue` _array_element_3))))
  (bind _outactors_4 (`GameplayStatics.GetAllActorsOfClass` "/Game/Gameplay/Objects/BP_DragonEgg.BP_DragonEgg_C"))
  (set `self.TotalEggs` (`KismetArrayLibrary.Array_Length` _outactors_4)))

(fn `UserConstructionScript`)