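; Game instance for Spark that owns the game's save data and session state such as current hub, checkpoint tag and menu-loading flag.
; On Init it loads or creates four save slots: user profile, collectibles, debug and GSR key-values.
; Profile events also apply subtitles, motion blur and sound-class volumes.
; Gem and egg GUIDs are stored per sublevel, then auto-saved asynchronously when the debug save enables it.
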(event `self.ReceiveInit`
  ;[1 1 1] Comment
  (`self.InitUserProfile`)
  (`self.InitCollectibleSave`)
  (`self.InitDebugSave`)
  (`self.InitGSRSave`))

(event `InitUserProfile`
  ;[1 1 1] User profile
  (bind _returnvalue (`GameplayStatics.DoesSaveGameExist` (`self.UserProfileSaveSlotName`)))
  (if _returnvalue
    (bind _returnvalue_2 (`GameplayStatics.LoadGameFromSlot` (`self.UserProfileSaveSlotName`)))
    (bind _asbp_spark_user_save (cast `/Game/Gameplay/SaveGame/BP_Spark_UserSave` _returnvalue_2))
    (set `self.UserProfileSaveGame` _asbp_spark_user_save)
    (else
      (bind _returnvalue_3 (`GameplayStatics.CreateSaveGameObject` "/Game/Gameplay/SaveGame/BP_Spark_UserSave.BP_Spark_UserSave_C"))
      (bind _output_get (set `self.UserProfileSaveGame` _returnvalue_3))
      (`GameplayStatics.SaveGameToSlot` _output_get (`self.UserProfileSaveSlotName`)))))

(event `SaveUserProfile`
  (params (SaveGame :type "SaveGame Object Reference"))
  (bind _spark_character_player (`/Game/Gameplay/Modes/BPFL_SparkGameModes.GetSparkPlayerCharacter`))
  ;[1 1 1] Comment
  (`GameplayStatics.SaveGameToSlot` SaveGame (`self.UserProfileSaveSlotName`))
  ;[1 1 1] Comment
  (`GameplayStatics.SetSubtitlesEnabled` (`/Game/Gameplay/SaveGame/BP_Spark_UserSave.ShowSubtitles` (`self.UserProfileSaveGame`)))
  (`/Engine/EditorBlueprintResources/StandardMacros.IsValid` _spark_character_player
    (:`Is Valid`
      (`/Game/Gameplay/Characters/Player/BP_SparkCharacter_Player.Set Motion Blur Enabled` _spark_character_player (`/Game/Gameplay/SaveGame/BP_Spark_UserSave.MotionBlur` (`self.UserProfileSaveGame`))))))

(event `RestoreUserProfile`
  ;[1 1 1] Comment
  (bind _returnvalue (`GameplayStatics.LoadGameFromSlot` (`self.UserProfileSaveSlotName`)))
  (bind _asbp_spark_user_save (cast `/Game/Gameplay/SaveGame/BP_Spark_UserSave` _returnvalue))
  (set `self.UserProfileSaveGame` _asbp_spark_user_save)
  ;[1 1 1] Comment
  (`/Game/Gameplay/Modes/BP_SparkGameModeBase.SetVolumeSoundClass` (`/Game/Gameplay/Modes/BPFL_SparkGameModes.GetSparkGameMode`) "NewEnumerator1" (`/Game/Gameplay/SaveGame/BP_Spark_UserSave.VolumeMaster` (`self.UserProfileSaveGame`)))
  (`/Game/Gameplay/Modes/BP_SparkGameModeBase.SetVolumeSoundClass` (`/Game/Gameplay/Modes/BPFL_SparkGameModes.GetSparkGameMode`) "NewEnumerator2" (`/Game/Gameplay/SaveGame/BP_Spark_UserSave.VolumeSFX` (`self.UserProfileSaveGame`)))
  (`/Game/Gameplay/Modes/BP_SparkGameModeBase.SetVolumeSoundClass` (`/Game/Gameplay/Modes/BPFL_SparkGameModes.GetSparkGameMode`) "NewEnumerator3" (`/Game/Gameplay/SaveGame/BP_Spark_UserSave.VolumeMusic` (`self.UserProfileSaveGame`)))
  (`/Game/Gameplay/Modes/BP_SparkGameModeBase.SetVolumeSoundClass` (`/Game/Gameplay/Modes/BPFL_SparkGameModes.GetSparkGameMode`) "NewEnumerator4" (`/Game/Gameplay/SaveGame/BP_Spark_UserSave.VolumeDialog` (`self.UserProfileSaveGame`))))

(event `ResetToDefaultUserProfile`
  ;[1 1 1] Comment
  (bind _returnvalue (`GameplayStatics.CreateSaveGameObject` "/Game/Gameplay/SaveGame/BP_Spark_UserSave.BP_Spark_UserSave_C"))
  (bind _output_get (set `self.UserProfileSaveGame` _returnvalue))
  (`GameplayStatics.SaveGameToSlot` _output_get (`self.UserProfileSaveSlotName`)))

(event `InitCollectibleSave`
  ;[1 1 1] Comment
  (bind _returnvalue (`GameplayStatics.DoesSaveGameExist` (`self.CollectibleSaveSlotName`)))
  (if _returnvalue
    (bind _returnvalue_2 (`GameplayStatics.LoadGameFromSlot` (`self.CollectibleSaveSlotName`)))
    (bind _asbp_spark_collectible_save (cast `/Game/Gameplay/SaveGame/BP_Spark_CollectibleSave` _returnvalue_2))
    (set `self.CollectibleSaveGame` _asbp_spark_collectible_save)
    (else
      (bind _returnvalue_3 (`GameplayStatics.CreateSaveGameObject` "/Game/Gameplay/SaveGame/BP_Spark_CollectibleSave.BP_Spark_CollectibleSave_C"))
      (bind _output_get (set `self.CollectibleSaveGame` _returnvalue_3))
      (`GameplayStatics.SaveGameToSlot` _output_get (`self.CollectibleSaveSlotName`)))))

(event `AutoSave`
  ;[1 1 1] c
  (if (`/Game/Gameplay/SaveGame/BP_Spark_DebugSave.EnableAutoSave` (`self.DebugSaveGame`))
    (`AsyncActionHandleSaveGame.AsyncSaveGameToSlot` (`self.CollectibleSaveGame`) (`self.CollectibleSaveSlotName`))))

(event `ResetCollectibleSave`
  ;[1 1 1] Comment
  (bind _returnvalue (`GameplayStatics.CreateSaveGameObject` "/Game/Gameplay/SaveGame/BP_Spark_CollectibleSave.BP_Spark_CollectibleSave_C"))
  (bind _output_get (set `self.CollectibleSaveGame` _returnvalue))
  (`GameplayStatics.SaveGameToSlot` _output_get (`self.CollectibleSaveSlotName`)))

(event `InitDebugSave`
  ;[1 1 1] Debug save
  (bind _returnvalue (`GameplayStatics.DoesSaveGameExist` (`self.DebugSaveSlotName`)))
  (if _returnvalue
    (bind _returnvalue_2 (`GameplayStatics.LoadGameFromSlot` (`self.DebugSaveSlotName`)))
    (bind _asbp_spark_debug_save (cast `/Game/Gameplay/SaveGame/BP_Spark_DebugSave` _returnvalue_2))
    (set `self.DebugSaveGame` _asbp_spark_debug_save)
    (else
      (bind _returnvalue_3 (`GameplayStatics.CreateSaveGameObject` "/Game/Gameplay/SaveGame/BP_Spark_DebugSave.BP_Spark_DebugSave_C"))
      (bind _output_get (set `self.DebugSaveGame` _returnvalue_3))
      (`GameplayStatics.SaveGameToSlot` _output_get (`self.DebugSaveSlotName`)))))

(event `SaveDebug`
  (params (SaveGame :type "SaveGame Object Reference"))
  ;[1 1 1] Comment
  (`GameplayStatics.SaveGameToSlot` SaveGame (`self.DebugSaveSlotName`)))

(event `ResetDebug`
  ;[1 1 1] Comment
  (bind _returnvalue (`GameplayStatics.LoadGameFromSlot` (`self.DebugSaveSlotName`)))
  (bind _asbp_spark_debug_save (cast `/Game/Gameplay/SaveGame/BP_Spark_DebugSave` _returnvalue))
  (set `self.DebugSaveGame` _asbp_spark_debug_save))

(event `InitGSRSave`
  ;[1 1 1] Comment
  (bind _returnvalue (`GameplayStatics.DoesSaveGameExist` (`self.GSRSaveSlotName`)))
  (if _returnvalue
    (bind _returnvalue_2 (`GameplayStatics.LoadGameFromSlot` (`self.GSRSaveSlotName`)))
    (bind _asbp_spark_gsrsave (cast `/Game/Gameplay/SaveGame/BP_Spark_GSRSave` _returnvalue_2))
    (set `self.GSRSaveGame` _asbp_spark_gsrsave)
    (else
      (bind _returnvalue_3 (`GameplayStatics.CreateSaveGameObject` "/Game/Gameplay/SaveGame/BP_Spark_GSRSave.BP_Spark_GSRSave_C"))
      (bind _output_get (set `self.GSRSaveGame` _returnvalue_3))
      (`GameplayStatics.SaveGameToSlot` _output_get (`self.GSRSaveSlotName`)))))

(event `SaveGSRValue`
  (params (GSRKey :type Name) (GSRValue :type Integer))
  ;[1 1 1] Comment
  (`BlueprintMapLibrary.Map_Add` (`/Game/Gameplay/SaveGame/BP_Spark_GSRSave.GSR` (`self.GSRSaveGame`)) GSRKey GSRValue)
  (`GameplayStatics.SaveGameToSlot` (`self.GSRSaveGame`) (`self.GSRSaveSlotName`)))

(fn `GetCheckpointTag`
  (returns (CheckpointTag :type String))
  (return (`self.CheckpointTag`)))

(fn `GetCurrentHubFileName`
  (returns (CurrentRealm :type Name))
  (return (`self.CurrentHubFileName`)))

(fn `GetLoadingToRootFromMenu`
  (returns (LoadingToRootFromMenu :type Boolean))
  (return (`self.LoadingToRootFromMenu`)))

(fn `IsItemCollected`
  (params (CollectibleType :type "/Game/Gameplay/SaveGame/ECollectibleType Enum" :default "NewEnumerator1") (ItemGUID :type "Guid Structure (by ref)"))
  (returns (ReturnValue :type Boolean))
  (locals (NewLocalVar_0 :type "/Game/Gameplay/SaveGame/SCollectibles Structure"))
  (bind _collectiblesavegame (`self.CollectibleSaveGame`))
  (bind _currentsublevelfilename (`/Game/Gameplay/Modes/BP_SparkGameState.GetCurrentSubLevelFileName` (`/Game/Gameplay/Modes/BPFL_SparkGameModes.GetSparkGameState`)))
  (return (`KismetArrayLibrary.Array_Contains` (`.CollectibleGUIDs_5_3A68D76245F2579E47BF618138C9355E` (break `/Game/Gameplay/SaveGame/SCollectibles` (select `/Game/Gameplay/SaveGame/ECollectibleType` CollectibleType :`NewEnumerator1` (`BlueprintMapLibrary.Map_Find` (`/Game/Gameplay/SaveGame/BP_Spark_CollectibleSave.Gems` _collectiblesavegame) _currentsublevelfilename) :`NewEnumerator2` (`BlueprintMapLibrary.Map_Find` (`/Game/Gameplay/SaveGame/BP_Spark_CollectibleSave.Eggs` _collectiblesavegame) _currentsublevelfilename)))) ItemGUID)))

(fn `SaveNewCollectible`
  (params (CollectibleType :type "/Game/Gameplay/SaveGame/ECollectibleType Enum" :default "NewEnumerator0") (CollectibleGUID :type "Guid Structure (by ref)"))
  (locals (LocalCurrentLevelCollected :type "Array of Guid Structure") (LocalCollectibleGUID :type "Guid Structure"))
  (bind _collectiblesavegame (`self.CollectibleSaveGame`))
  (bind _currentsublevelfilename (`/Game/Gameplay/Modes/BP_SparkGameState.GetCurrentSubLevelFileName` (`/Game/Gameplay/Modes/BPFL_SparkGameModes.GetSparkGameState`)))
  (set `local.LocalCollectibleGUID` CollectibleGUID)
  (bind _output_get (set `local.LocalCurrentLevelCollected` (`.CollectibleGUIDs_5_3A68D76245F2579E47BF618138C9355E` (break `/Game/Gameplay/SaveGame/SCollectibles` (select `/Game/Gameplay/SaveGame/ECollectibleType` CollectibleType :`NewEnumerator1` (`BlueprintMapLibrary.Map_Find` (`/Game/Gameplay/SaveGame/BP_Spark_CollectibleSave.Gems` _collectiblesavegame) _currentsublevelfilename) :`NewEnumerator2` (`BlueprintMapLibrary.Map_Find` (`/Game/Gameplay/SaveGame/BP_Spark_CollectibleSave.Eggs` _collectiblesavegame) _currentsublevelfilename))))))
  (`KismetArrayLibrary.Array_Add` _output_get (`local.LocalCollectibleGUID`))
  (switch `/Game/Gameplay/SaveGame/ECollectibleType` CollectibleType
    (:`NewEnumerator1`
      (`BlueprintMapLibrary.Map_Add` (`/Game/Gameplay/SaveGame/BP_Spark_CollectibleSave.Gems` (`self.CollectibleSaveGame`)) (`/Game/Gameplay/Modes/BP_SparkGameState.GetCurrentSubLevelFileName` (`/Game/Gameplay/Modes/BPFL_SparkGameModes.GetSparkGameState`)) (make `/Game/Gameplay/SaveGame/SCollectibles` (`local.LocalCurrentLevelCollected`))))
    (:`NewEnumerator2`
      (`BlueprintMapLibrary.Map_Add` (`/Game/Gameplay/SaveGame/BP_Spark_CollectibleSave.Eggs` (`self.CollectibleSaveGame`)) (`/Game/Gameplay/Modes/BP_SparkGameState.GetCurrentSubLevelFileName` (`/Game/Gameplay/Modes/BPFL_SparkGameModes.GetSparkGameState`)) (make `/Game/Gameplay/SaveGame/SCollectibles` (`local.LocalCurrentLevelCollected`)))))
  (`self.AutoSave`))

(fn `Set Checkpoint`
  (params (CheckpointTag :type "PlayerStart Object Reference"))
  (set `self.CheckpointTag` (`KismetStringLibrary.Conv_NameToString` (`PlayerStart.PlayerStartTag` CheckpointTag))))

(fn `SetCurrentHubFileName`
  (params (CurrentRealm :type Name))
  (set `self.CurrentHubFileName` CurrentRealm))

(fn `SetLoadingToRootFromMenu`
  (params (LoadingToRootFromMenu :type Boolean))
  (set `self.LoadingToRootFromMenu` LoadingToRootFromMenu))