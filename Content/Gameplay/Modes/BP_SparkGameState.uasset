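; Game state for Spark that tracks gem and egg counts for the current level, plus its sub-level file name.
; Increment functions save each collectible by GUID through the Spark game instance, update the count and broadcast new and previous values.
; The level's gem total sums placed gems and chest contents; the loop over AI characters is an empty stub.
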(fn `GetCurrentLevelEggCount`
  (returns (EggCount :type Integer))
  (return (`self.EggCount`)))

(fn `GetCurrentLevelGemCount`
  (returns (CurrentLevelGemCount :type Integer))
  (return (`self.CurrentLevelGemCount`)))

(fn `GetCurrentLevelTotalGemCount`
  (returns (CurrentLevelGemTotalCount :type Integer))
  (return (`self.CurrentLevelGemTotalCount`)))

(fn `GetCurrentSubLevelFileName`
  (returns (CurrentSubLevelFileName :type Name))
  (return (`self.CurrentSubLevelFileName`)))

(fn `IncrementCurrentEggCount`
  (params (GemGUID :type "Guid Structure (by ref)"))
  (returns (NewEggCount :type Integer))
  (locals (LocalPreviousEggCount :type Integer :default 0))
  (`/Game/Gameplay/Modes/BP_SparkGameInstance.SaveNewCollectible` (`/Game/Gameplay/Modes/BPFL_SparkGameModes.GetSparkGameInstance`) "NewEnumerator2" GemGUID)
  (bind _output_get (set `local.LocalPreviousEggCount` (`self.EggCount`)))
  (set `self.EggCount` (+ _output_get 1))
  (`self.OnCurrentLevelEggCountChanged` (`self.EggCount`) (`local.LocalPreviousEggCount`))
  (return (`self.EggCount`)))

(fn `IncrementCurrentLevelGemCount`
  (params (IncrementAmount :type Integer) (GUID :type "Guid Structure"))
  (returns (NewAmount :type Integer))
  (locals (LocalPreviousGemCount :type Integer))
  (bind _currentlevelgemcount (`self.CurrentLevelGemCount`))
  (`/Game/Gameplay/Modes/BP_SparkGameInstance.SaveNewCollectible` (`/Game/Gameplay/Modes/BPFL_SparkGameModes.GetSparkGameInstance`) "NewEnumerator1" GUID)
  (set `local.LocalPreviousGemCount` _currentlevelgemcount)
  (bind _output_get (set `self.CurrentLevelGemCount` (+ IncrementAmount _currentlevelgemcount)))
  (`self.OnCurrentLevelGemCountChanged` _output_get (`local.LocalPreviousGemCount`))
  (return _output_get))

(fn `SetCurrentLevelGemCountMax`
  ;[1 1 1] Placed gems
  (bind _outactors (`GameplayStatics.GetAllActorsOfClass` "/Game/Gameplay/Objects/BP_Gem.BP_Gem_C"))
  (for _array_element _outactors
    (set `self.CurrentLevelGemTotalCount` (+ (`self.CurrentLevelGemTotalCount`) (`/Game/Gameplay/Objects/BP_Gem.GetGemValue` _array_element))))
  ;[1 1 1] Gems in chests
  (bind _outactors_2 (`GameplayStatics.GetAllActorsOfClass` "/Game/Gameplay/Objects/BP_Chest.BP_Chest_C"))
  (for _array_element_2 _outactors_2
    (set `self.CurrentLevelGemTotalCount` (+ (`self.CurrentLevelGemTotalCount`) (`/Game/Gameplay/Objects/BP_Chest.GetContainedTotalGemValue` _array_element_2))))
  ;[1 1 1] Gems in characters
  (bind _outactors_3 (`GameplayStatics.GetAllActorsOfClass` "/Game/Gameplay/Characters/AI/BP_SparkCharacter_AI.BP_SparkCharacter_AI_C"))
  (for _ _outactors_3
    _))

(fn `SetCurrentSubLevelFileName`
  (params (CurrentSubLevelFileName :type Name))
  (set `self.CurrentSubLevelFileName` CurrentSubLevelFileName)
  (return))

(fn `UserConstructionScript`)